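; Behavior Tree task that moves a zombie AI's controlled pawn to the actor stored in its TargetToFollow blackboard key.
; It casts the owner to BP_ZombieAI_Controller on first use and caches it, then runs AIMoveTo with a small fixed acceptance radius.
; Only a successful move finishes the task; a failed move or failed cast never calls FinishExecute.
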(event EventReceiveExecute
  (params (OwnerActor :type Actor%20Object%20Reference))
  ;[1 1 1] If the AI has a controller move to the desired location.
  (if (!= (Variables|Default|GetAI_Con_Ref) 0)
    _
    (else
      (bind _asbp_zombie_ai_controller (Utilities|Casting|CastToBP_ZombieAI_Controller OwnerActor))
      (Variables|Default|SetAI_Con_Ref _asbp_zombie_ai_controller)))
  (AI|AIMoveTo (Pawn|GetControlledPawn (Variables|Default|GetAI_Con_Ref)) "0, 0, 0" (AI|BehaviorTree|GetBlackboardValueasActor (Variables|Default|GetTargetToFollow)) 5e+01 false
    (:OnSuccess
      (AI|BehaviorTree|FinishExecute true))))