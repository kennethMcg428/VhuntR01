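; Behavior tree decorator for the zombie AI that gates a branch on the pawn's distance to its follow target.
; It measures the distance between the controlled pawn and the TargetToFollow actor and writes it to the DistanceToTarget blackboard key.
; Despite its name, the check passes when that distance is at least AcceptableDistance.
; It fails with a printed error if the owner is not a BP_ZombieAI_Controller.
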(fn PerformConditionCheck
  (params (OwnerActor :type Actor%20Object%20Reference))
  ;[1 1 1] Check to see if the AI is closer than the acceptable distance and then pass a success.
  (bind _asbp_zombie_ai_controller (Utilities|Casting|CastToBP_ZombieAI_Controller OwnerActor)
    (:then
      (Variables|Default|SetAI_Con_Ref _asbp_zombie_ai_controller)
      (Class|BTFunctionLibrary|SetBlackboardValueasFloat (Variables|Default|GetDistanceToTarget) (Math|Vector|VectorLength (- (Transformation|GetActorLocation (AI|BehaviorTree|GetBlackboardValueasActor (Variables|Default|GetTargetToFollow))) (Transformation|GetActorLocation (Pawn|GetControlledPawn (Variables|Default|GetAI_Con_Ref))))))
      (return (>= (Math|Vector|VectorLength (- (Transformation|GetActorLocation (AI|BehaviorTree|GetBlackboardValueasActor (Variables|Default|GetTargetToFollow))) (Transformation|GetActorLocation (Pawn|GetControlledPawn (Variables|Default|GetAI_Con_Ref))))) (Variables|Default|GetAcceptableDistance))))
    (:CastFailed
      (Development|PrintString "Error: CloseEnough:No AI Controller" false)
      (return false))))