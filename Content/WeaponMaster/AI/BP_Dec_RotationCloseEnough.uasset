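; Behavior tree decorator for zombie AI that checks how far the controlled pawn faces away from its follow target.
; It computes the absolute yaw difference between the pawn's rotation and the look-at rotation to TargetToFollow, writing it to the RotationToTarget blackboard key.
; Despite the RotationCloseEnough name, it passes only when that difference exceeds a fixed threshold.
; Without a BP_ZombieAI_Controller owner, it prints an error and fails.
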(fn PerformConditionCheck
  (params (OwnerActor :type Actor%20Object%20Reference))
  ;[1 1 1] See if the angle to the target to follow is close enough and then pass success.
  (bind _asbp_zombie_ai_controller (Utilities|Casting|CastToBP_ZombieAI_Controller OwnerActor)
    (:then
      (Variables|Default|SetAI_Con_Ref _asbp_zombie_ai_controller)
      (Class|BTFunctionLibrary|SetBlackboardValueasFloat (Variables|Default|GetRotationToTarget) (Math|Float|Absolute(Float) (.Yaw (Math|Rotator|BreakRotator (Math|Rotator|Delta(Rotator) (Math|Rotator|FindLookatRotation (Transformation|GetActorLocation (Pawn|GetControlledPawn (Variables|Default|GetAI_Con_Ref))) (Transformation|GetActorLocation (AI|BehaviorTree|GetBlackboardValueasActor (Variables|Default|GetTargetToFollow)))) (Transformation|GetActorRotation (Pawn|GetControlledPawn (Variables|Default|GetAI_Con_Ref))))))))
      (return (> (Math|Float|Absolute(Float) (.Yaw (Math|Rotator|BreakRotator (Math|Rotator|Delta(Rotator) (Math|Rotator|FindLookatRotation (Transformation|GetActorLocation (Pawn|GetControlledPawn (Variables|Default|GetAI_Con_Ref))) (Transformation|GetActorLocation (AI|BehaviorTree|GetBlackboardValueasActor (Variables|Default|GetTargetToFollow)))) (Transformation|GetActorRotation (Pawn|GetControlledPawn (Variables|Default|GetAI_Con_Ref))))))) 2e+01)))
    (:CastFailed
      (Development|PrintString "Error: RotationCloseEnough: No AI Controller" false)
      (return false))))