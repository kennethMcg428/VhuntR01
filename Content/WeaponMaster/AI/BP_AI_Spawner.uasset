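; AI spawner actor that periodically spawns melee AI zombies with a behavior tree at its own transform.
; A looping SpawnRate timer runs TrySpawn, which either keeps a single living zombie of its own or defers to BP_SurvivalGameMode when UseGameMode is set.
; In game mode, it asks CheckCanSpawn, waits a random delay to vary animations, then spawns and reports the zombie via ZombieSpawned.
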(event Custom|TrySpawn
  (bind _returnvalue (Transformation|GetActorTransform))
  (bind _returnvalue_2 (Transformation|GetActorTransform))
  (bind (_location _rotation) (Math|Transform|BreakTransform _returnvalue))
  (bind (_location_2 _rotation_2) (Math|Transform|BreakTransform _returnvalue_2))
  ;[1 1 1] We will try to spawn based on spawn rate. If UseGameMode is true then the game mode will decide if we can spawn, else the spawner will only spawn one zombie at a time.
  (if (not (Variables|SpawnerSetup|GetbUseGameMode))
    (Utilities|IsValid (Variables|DoNotTouch|GetCurrentZombie)
      (:Is%20Valid
        (if (Variables|/Game/WeaponMaster/AI/BP_MeleeAI_Character.BP_MeleeAI_Character_C|GetbIsDead (Variables|DoNotTouch|GetCurrentZombie))
          (Variables|DoNotTouch|SetCurrentZombie 0)
          (bind _returnvalue_3 (AI|SpawnAIFromClass (Variables|SpawnerSetup|GetAIToSpawn) (Variables|SpawnerSetup|GetBehaviorTree) _location _rotation false :!label _label))
          (bind _asbp_melee_ai_character (Utilities|Casting|CastToBP_MeleeAI_Character _returnvalue_3))
          (Variables|DoNotTouch|SetCurrentZombie _asbp_melee_ai_character)))
      (:Is%20Not%20Valid
        (goto _label)))
    (else
      (Utilities|IsValid (Variables|DoNotTouch|GetSurvivalGameMode)
        (:Is%20Valid
          (if (CallFunction|CanSpawn)
            ;;[1 1 1] Delay to get animation variation
            (Utilities|FlowControl|Delay (Math|Random|RandomFloatinRange 0.5 (- (Variables|SpawnerSetup|GetSpawnRate) 0.5)))
            (bind _returnvalue_4 (AI|SpawnAIFromClass (Variables|SpawnerSetup|GetAIToSpawn) (Variables|SpawnerSetup|GetBehaviorTree) _location_2 _rotation_2 false))
            (bind _asbp_melee_ai_character_2 (Utilities|Casting|CastToBP_MeleeAI_Character _returnvalue_4))
            (Utilities|IsValid _asbp_melee_ai_character_2
              (:Is%20Valid
                (Default|ZombieSpawned (Variables|DoNotTouch|GetSurvivalGameMode) _asbp_melee_ai_character_2)))))))))

(event EventBeginPlay
  ;[1 1 1] We need to know if we are using the survival game mode or not.
  (bind _asbp_survival_game_mode (Utilities|Casting|CastToBP_SurvivalGameMode (Game|GetGameMode))
    (:then
      (Variables|DoNotTouch|SetSurvivalGameMode _asbp_survival_game_mode))
    (:CastFailed
      _))
  (Utilities|Time|SetTimerbyEvent (delegate Custom|TrySpawn) (Variables|SpawnerSetup|GetSpawnRate) true))

(event Collision|EventActorBeginOverlap
  (params (OtherActor :type Actor%20Object%20Reference)))

(event EventTick
  (params (DeltaSeconds :type Float%20%28single-precision%29)))

(fn ConstructionScript)

(fn CanSpawn
  ;[1 1 1] Checkto see if the gamemode is ready for another zombie.
  (bind _bcanspawn (Default|CheckCanSpawn (Variables|DoNotTouch|GetSurvivalGameMode)))
  (return _bcanspawn))