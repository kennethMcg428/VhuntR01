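; Behavior tree task that tells a melee AI character to stop attacking.
; On execute it caches the controlled pawn as a BP_MeleeAI_Character if no reference is stored, then sets a CanAttack flag.
; With that flag set, the AI tick calls StopAttack if the character's CanStopAttack allows it, and finishes successfully either way.
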(event EventReceiveTickAI
  (params (OwnerController :type AI%20Controller%20Object%20Reference) (ControlledPawn :type Pawn%20Object%20Reference) (DeltaSeconds :type Float%20%28single-precision%29))
  (bind _ai_car_ref (Variables|Default|GetAI_Car_Ref))
  ;[1 1 1] If can attack, on tick start attack.
  (if (Variables|Default|GetbCanAttack)
    (if (Variables|/Game/WeaponMaster/AI/BP_MeleeAI_Character.BP_MeleeAI_Character_C|GetbCanStopAttack _ai_car_ref)
      (Default|StopAttack _ai_car_ref))
    (AI|BehaviorTree|FinishExecute true)))

(event EventReceiveExecuteAI
  (params (OwnerController :type AI%20Controller%20Object%20Reference) (ControlledPawn :type Pawn%20Object%20Reference))
  ;[1 1 1] On execute make sure there is a controller reference and set can attack to true.
  (if (!= (Variables|Default|GetAI_Car_Ref) 0)
    _
    (else
      (bind _asbp_melee_ai_character (Utilities|Casting|CastToBP_MeleeAI_Character ControlledPawn))
      (Variables|Default|SetAI_Car_Ref _asbp_melee_ai_character)))
  (Variables|Default|SetbCanAttack true))