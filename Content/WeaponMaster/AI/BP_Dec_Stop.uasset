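; Behavior tree decorator for zombie AI that passes while the pawn is at least an acceptable distance from its follow target.
; It casts the owner to BP_ZombieAI_Controller and caches that reference.
; It then compares the distance between the controlled pawn and the TargetToFollow blackboard actor against AcceptableDistance.
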(fn PerformConditionCheck
  (params (OwnerActor :type Actor%20Object%20Reference))
  (bind _asbp_zombie_ai_controller (Utilities|Casting|CastToBP_ZombieAI_Controller OwnerActor))
  (Variables|Default|SetAI_Con_Ref _asbp_zombie_ai_controller)
  (return (>= (Math|Vector|VectorLength (- (Transformation|GetActorLocation (AI|BehaviorTree|GetBlackboardValueasActor (Variables|Default|GetTargetToFollow))) (Transformation|GetActorLocation (Pawn|GetControlledPawn (Variables|Default|GetAI_Con_Ref))))) (Variables|Default|GetAcceptableDistance))))