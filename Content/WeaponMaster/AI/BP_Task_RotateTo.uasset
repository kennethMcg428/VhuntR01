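; Behavior Tree task that turns the controlled melee AI character to face the actor in the TargetToFollow blackboard key.
; On execute it caches the zombie AI controller and character, then enables rotation, printing a message if either cast fails.
; Each tick interpolates only the pawn's yaw toward the target.
; It finishes successfully when the rotation nearly matches the full look-at rotation, pitch included.
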(event EventReceiveTickAI
  (params (OwnerController :type AI%20Controller%20Object%20Reference) (ControlledPawn :type Pawn%20Object%20Reference) (DeltaSeconds :type Float%20%28single-precision%29))
  (bind _ai_con_ref (Variables|Default|GetAI_Con_Ref))
  (bind _targettofollow (Variables|Default|GetTargetToFollow))
  (bind _returnvalue (Pawn|GetControlledPawn _ai_con_ref))
  (bind _returnvalue_2 (AI|BehaviorTree|GetBlackboardValueasActor _targettofollow))
  (bind _returnvalue_3 (Transformation|GetActorLocation _returnvalue_2))
  (bind _returnvalue_4 (Transformation|GetActorLocation _returnvalue))
  (bind _returnvalue_5 (Transformation|GetActorRotation _returnvalue))
  (bind _returnvalue_6 (Math|Rotator|FindLookatRotation _returnvalue_4 _returnvalue_3))
  ;[1 1 1] Rotate the character towards the target actor.
  (if (Variables|Default|GetCanRotate)
    (Transformation|SetActorRotation _returnvalue (Math|Interpolation|RInterpTo _returnvalue_5 (Math|Rotator|MakeRotator 0.0 0.0 (.Yaw (Math|Rotator|BreakRotator _returnvalue_6))) DeltaSeconds 7.0))
    (if (Math|Rotator|Equal(Rotator) _returnvalue_5 _returnvalue_6 0.1)
      (AI|BehaviorTree|FinishExecute true))))

(event EventReceiveExecuteAI
  (params (OwnerController :type AI%20Controller%20Object%20Reference) (ControlledPawn :type Pawn%20Object%20Reference))
  ;[1 1 1] Make sure we have both a controller and a character then set Can rotate to true.
  (if (!= (Variables|Default|GetAI_Con_Ref) 0)
    (if (!= (Variables|Default|GetAI_Car_Ref) 0) :!label _label
      (Variables|Default|SetCanRotate true :!label _label_2)
      (else
        (bind _asbp_melee_ai_character (Utilities|Casting|CastToBP_MeleeAI_Character ControlledPawn)
          (:then
            (Variables|Default|SetAI_Car_Ref _asbp_melee_ai_character)
            (goto _label_2))
          (:CastFailed
            (Development|PrintString "No Character" false)))))
    (else
      (bind _asbp_zombie_ai_controller (Utilities|Casting|CastToBP_ZombieAI_Controller OwnerController)
        (:then
          (Variables|Default|SetAI_Con_Ref _asbp_zombie_ai_controller)
          (goto _label))
        (:CastFailed
          (Development|PrintString "No Controller" false))))))