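; Base melee AI zombie character for survival mode that attacks, takes damage and reports kills and headshots to BP_SurvivalGameMode.
; Attack events play a montage, mute idle audio and drive a forward capsule trace that applies melee damage.
; Point and radial damage reduce health, set the Blackboard Dead key, then ragdoll with optional impulse and timed destroy, either immediately or via death-animation notifies.
; Construction script reapplies mesh and AnimBP, working around a child-Blueprint engine bug.
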(event Custom|StartAttack
  ;[1 1 1] Attacking
  (Variables|DoNotTouch|SetbIsAttacking true)
  (Audio|Components|Audio|AdjustVolume (Variables|Default|GetZombieIdle) 0.0 0.0 :!class /Script/Engine.AudioComponent)
  (Animation|PlayAnimMontage (Variables|AISetup|GetAttackAnimMontage) 1.0 "None"))

(event Custom|RadialDamageRagdoll
  (bind _mesh (Variables|Character|GetMesh))
  ;[1 1 1] TakeDamage
  ;;[0 0 0] Call this using a Anim Notify in the death animation
  ;;[0 0 0] If we don't want to ragdoll after the death animation lets destroy the actor, else lets ragdoll.
  (if (not (Variables|AISetup|GetbUseRagdollDuringDeathAnimation))
    _
    (else
      ;;[0 0 0] Ragdoll
      (Collision|SetCollisionEnabled _mesh "QueryAndPhysics")
      (Physics|SetSimulatePhysics _mesh true)
      (Audio|Components|Audio|Stop (Variables|Default|GetZombieIdle))
      (Collision|SetCollisionEnabled (Variables|Collision|GetCapsuleComponent) "NoCollision")
      ;;[0 0 0] Should we add an impulse?
      (if (not (Variables|AISetup|GetbApplyImpulseOnDeath))
        _
        (else
          ;;[0 0 0] Add Impulse
          (Physics|AddImpulse (Variables|Character|GetMesh) (* (Math|Vector|GetUnitDirection(Vector) (stale Game|Damage|EventRadialDamage Origin) (Transformation|GetActorLocation)) (* (Variables|/Script/Engine.DamageType|GetDamageImpulse (stale Game|Damage|EventRadialDamage DamageType)) 2e+01)) "None" false)))))
  ;;[0 0 0] Should we destroy?
  (if (Variables|AISetup|GetbDestroyOnDeath)
    (Utilities|Time|SetTimerbyEvent (delegate Custom|DestroyZombie) 5.0)))

(event Custom|PlayAttackSound
  ;[1 1 1] Attacking
  (if (not (Variables|DoNotTouch|GetbIsDead))
    (Audio|PlaySoundatLocation (Variables|AISetup|GetAttackSound) (Transformation|GetWorldLocation (Variables|Collision|GetCapsuleComponent)))))

(event Custom|PointDamageRagdoll
  (bind _mesh (Variables|Character|GetMesh))
  (bind _mesh_2 (Variables|Character|GetMesh))
  ;[1 1 1] TakeDamage
  ;;[0 0 0] Call this using a Anim Notify in the Point Damange death animation
  ;;[0 0 0] If we don't want to ragdoll after the death animation lets destroy the actor, else lets ragdoll.
  (if (not (Variables|AISetup|GetbUseRagdollDuringDeathAnimation))
    _
    (else
      ;;[0 0 0] Ragdoll
      (Collision|SetCollisionEnabled _mesh "QueryAndPhysics")
      (Physics|SetSimulatePhysics _mesh true)
      (Audio|Components|Audio|Stop (Variables|Default|GetZombieIdle))
      (Collision|SetCollisionEnabled (Variables|Collision|GetCapsuleComponent) "NoCollision")
      ;;[0 0 0] Should we add an impulse?
      (if (not (Variables|AISetup|GetbApplyImpulseOnDeath))
        _
        (else
          ;;[0 0 0] Add Impulse
          (if (== (stale Game|Damage|EventPointDamage DamageType) "/Game/WeaponMaster/Blueprints/Weapons/DamageTypes/BP_DT_Melee.BP_DT_Melee_C")
            (Physics|AddImpulseatLocation _mesh_2 (* (stale Game|Damage|EventPointDamage ShotFromDirection) (Variables|/Script/Engine.DamageType|GetDamageImpulse (stale Game|Damage|EventPointDamage DamageType))) (stale Game|Damage|EventPointDamage HitLocation) "None")
            (else
              (Physics|AddImpulseatLocation _mesh_2 (* (stale Game|Damage|EventPointDamage ShotFromDirection) (* (Variables|/Script/Engine.DamageType|GetDamageImpulse (stale Game|Damage|EventPointDamage DamageType)) 1e+01)) (stale Game|Damage|EventPointDamage HitLocation) "None")))))))
  ;;[0 0 0] Should we destroy?
  (if (Variables|AISetup|GetbDestroyOnDeath)
    (Utilities|Time|SetTimerbyEvent (delegate Custom|DestroyZombie) 5.0)))

(event Custom|StartSwing
  ;[1 1 1] Attacking
  (if (not (Variables|DoNotTouch|GetbIsDead))
    (CallFunction|AttackCast)))

(event Custom|StopAttack
  ;[1 1 1] Attacking
  (Animation|StopAnimMontage (Variables|AISetup|GetAttackAnimMontage))
  (Variables|DoNotTouch|SetbIsAttacking false)
  (AI|Components|Blackboard|SetValueasBool (Variables|Default|GetBlackboardComponent) (Variables|AISetup|GetAttacking) false)
  (bind _returnvalue (Utilities|Time|SetTimerbyEvent (delegate Custom|RestartIdleSound) 2.0)))

(event Custom|DestroyZombie
  ;[1 1 1] TakeDamage
  ;;[0 0 0] Destroy AI
  (Actor|DestroyActor))

(event Custom|RestartIdleSound
  ;[1 1 1] Attacking
  (if (not (Variables|DoNotTouch|GetbIsAttacking))
    (Audio|Components|Audio|AdjustVolume (Variables|Default|GetZombieIdle) 0.0 1.0 :!class /Script/Engine.AudioComponent)
    (Utilities|Time|ClearandInvalidateTimerbyHandle (stale Custom|StopAttack _returnvalue))))

(event EventBeginPlay
  ;[1 1 1] BeginPlay
  (bind _blackboardcomponent (Class|AIController|UseBlackboard (AI|GetAIController (Pawn|GetController)) (Variables|AISetup|GetBlackBoard)))
  (bind _output_get (Variables|Default|SetBlackboardComponent _blackboardcomponent))
  (AI|Components|Blackboard|SetValueasVector _output_get (Variables|AISetup|GetHomeLocation) (Transformation|GetActorLocation)))

(event Game|Damage|EventPointDamage
  (params (Damage :type Float%20%28single-precision%29) (DamageType :type Damage%20Type%20Object%20Reference) (HitLocation :type Vector) (HitNormal :type Vector :default "0, 0, 0") (HitComponent :type Primitive%20Component%20Object%20Reference) (BoneName :type Name :default "None") (ShotFromDirection :type Vector) (InstigatedBy :type Controller%20Object%20Reference) (DamageCauser :type Actor%20Object%20Reference) (HitInfo :type Hit%20Result%20Structure%20%28by%20ref%29))
  (bind _mesh (Variables|Character|GetMesh))
  (bind _damageimpulse (Variables|/Script/Engine.DamageType|GetDamageImpulse DamageType))
  (bind _mesh_2 (Variables|Character|GetMesh))
  ;[1 1 1] TakeDamage
  (if (not (Variables|DoNotTouch|GetbIsDead))
    (bind _output_get (Variables|AISetup|SetHealth (- (Variables|AISetup|GetHealth) Damage)))
    (if (<= _output_get 0.0)
      ;;[0 0 0] Set Dead
      (Variables|DoNotTouch|SetbIsDead true)
      (AI|Components|Blackboard|SetValueasBool (Variables|Default|GetBlackboardComponent) (Variables|AISetup|GetDead) true)
      (switch Utilities|FlowControl|Switch|SwitchonEPhysicalSurface (Variables|/Script/Engine.PhysicalMaterial|GetSurfaceType (.PhysMat (Collision|BreakHitResult HitInfo)))
        (:SurfaceType_Default
          ;;[0 0 0] Increment Score
          (CallFunction|IncrementScore false :!label _label))
        (:SurfaceType1
          (goto _label))
        (:SurfaceType5
          (goto _label))
        (:SurfaceType7
          (CallFunction|IncrementScore true)))
      ;;[0 0 0] If we are not using a death animation lets do a ragdoll, else we will let the death animation handle it.
      (if (not (Variables|AISetup|GetbUseDeathAnimation))
        ;;[0 0 0] Ragdoll
        (Collision|SetCollisionEnabled _mesh "QueryAndPhysics")
        (Physics|SetSimulatePhysics _mesh true)
        (Audio|Components|Audio|Stop (Variables|Default|GetZombieIdle))
        (Collision|SetCollisionEnabled (Variables|Collision|GetCapsuleComponent) "NoCollision")
        ;;[0 0 0] Should we add an impulse?
        (if (not (Variables|AISetup|GetbApplyImpulseOnDeath))
          _
          (else
            ;;[0 0 0] Add Impulse
            (if (== DamageType "/Game/WeaponMaster/Blueprints/Weapons/DamageTypes/BP_DT_Melee.BP_DT_Melee_C")
              (Physics|AddImpulseatLocation _mesh_2 (* ShotFromDirection _damageimpulse) HitLocation "None")
              (else
                (Physics|AddImpulseatLocation _mesh_2 (* ShotFromDirection (* _damageimpulse 1e+01)) HitLocation "None")))))
        ;;[0 0 0] Should we destroy?
        (if (Variables|AISetup|GetbDestroyOnDeath)
          (Utilities|Time|SetTimerbyEvent (delegate Custom|DestroyZombie) 5.0))))))

(event Game|Damage|EventRadialDamage
  (params (DamageReceived :type Float%20%28single-precision%29) (DamageType :type Damage%20Type%20Object%20Reference) (Origin :type Vector) (HitInfo :type Hit%20Result%20Structure%20%28by%20ref%29) (InstigatedBy :type Controller%20Object%20Reference) (DamageCauser :type Actor%20Object%20Reference))
  (bind _mesh (Variables|Character|GetMesh))
  ;[1 1 1] TakeDamage
  (if (not (Variables|DoNotTouch|GetbIsDead))
    (bind _output_get (Variables|AISetup|SetHealth (- (Variables|AISetup|GetHealth) DamageReceived)))
    (if (<= _output_get 0.0)
      ;;[0 0 0] Set Dead
      (Variables|DoNotTouch|SetbIsDead true)
      (AI|Components|Blackboard|SetValueasBool (Variables|Default|GetBlackboardComponent) (Variables|AISetup|GetDead) true)
      ;;[0 0 0] Increment Score
      (CallFunction|IncrementScore false)
      ;;[0 0 0] If we are not using a death animation lets do a ragdoll, else we will let the death animation handle it.
      (if (not (Variables|AISetup|GetbUseDeathAnimation))
        ;;[0 0 0] Ragdoll
        (Collision|SetCollisionEnabled _mesh "QueryAndPhysics")
        (Physics|SetSimulatePhysics _mesh true)
        (Audio|Components|Audio|Stop (Variables|Default|GetZombieIdle))
        (Collision|SetCollisionEnabled (Variables|Collision|GetCapsuleComponent) "NoCollision")
        ;;[0 0 0] Should we add an impulse?
        (if (not (Variables|AISetup|GetbApplyImpulseOnDeath))
          _
          (else
            ;;[0 0 0] Add Impulse
            (Physics|AddImpulse (Variables|Character|GetMesh) (* (Math|Vector|GetUnitDirection(Vector) Origin (Transformation|GetActorLocation)) (* (Variables|/Script/Engine.DamageType|GetDamageImpulse DamageType) 2e+01)) "None" false)))
        ;;[0 0 0] Should we destroy?
        (if (Variables|AISetup|GetbDestroyOnDeath)
          (Utilities|Time|SetTimerbyEvent (delegate Custom|DestroyZombie) 5.0))))))

(fn ConstructionScript
  (bind _mesh (Variables|Character|GetMesh))
  ;[1 1 1] Manually set mesh and animation blueprint to get around Engine Bug that resets child blueprint mesh values
  (Class|SkinnedMeshComponent|SetSkeletalMesh (Variables|Character|GetMesh) (Variables|AISetup|GetAIMesh) true)
  (Components|SkeletalMesh|SetAnimInstanceClass _mesh (Variables|AISetup|GetAI_AnimBlueprint))
  (Variables|/Script/Engine.PrimitiveComponent|SetbGenerateOverlapEvents _mesh true)
  (Collision|SetCollisionObjectType _mesh "ECC_PhysicsBody"))

(fn IncrementScore
  (params (HeadShot :type Boolean))
  ;[1 1 1] Tell the gamemode to increase the players score.
  (bind _asbp_survival_game_mode (Utilities|Casting|CastToBP_SurvivalGameMode (Game|GetGameMode))
    (:then
      (Default|ZombieKilled _asbp_survival_game_mode HeadShot))
    (:CastFailed
      (Development|PrintString "IncorrectGameMode" false))))

(fn AttackCast
  (bind _capsulecomponent (Variables|Collision|GetCapsuleComponent))
  (bind _returnvalue (Transformation|GetWorldLocation _capsulecomponent))
  ;[1 1 1] Check to see if the player is within a capsule area of the AI and then deal damage.
  (bind _outhit (Class|KismetSystemLibrary|CapsuleTraceSingleforObjects _returnvalue (+ _returnvalue (* (Transformation|GetActorForwardVector) 1e+02)) 45.0 6e+01 (Variables|AISetup|GetObjectsToHitscanFor) false (Utilities|Array|MakeArray self) "None" true))
  (if (and (.bBlockingHit (Collision|BreakHitResult _outhit)) (not (Variables|DoNotTouch|GetbIsDead)))
    (Game|Damage|ApplyDamage (.HitActor (Collision|BreakHitResult _outhit)) (Variables|AISetup|GetDamagePerHit) (Pawn|GetController) self "/Game/WeaponMaster/Blueprints/Weapons/DamageTypes/BP_DT_Melee.BP_DT_Melee_C")))