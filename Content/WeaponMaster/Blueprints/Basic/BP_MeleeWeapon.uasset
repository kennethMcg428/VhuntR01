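; Grabbable, holsterable melee weapon that deals swing damage based on hit box velocity.
; Overlaps above a minimum speed trigger a sphere trace from the trace socket, and DoHit picks surface-specific decals, effects and sounds before point damage is applied.
; Flesh and cloth damage scales with capped speed, and head hits add a critical multiplier.
; Trigger input toggles an optional secondary hold, which Tick interpolates into place before allowing another swap.
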(event OnComponentBeginOverlap(HitBox)
  (params (OverlappedComponent :type Primitive%20Component%20Object%20Reference) (OtherActor :type Actor%20Object%20Reference) (OtherComp :type Primitive%20Component%20Object%20Reference) (OtherBodyIndex :type Integer) (bFromSweep :type Boolean) (SweepResult :type Hit%20Result%20Structure%20%28by%20ref%29))
  (bind _maximumswingspeed (Variables|MeleeWeaponSetup|GetMaximumSwingSpeed))
  (bind _skeletalmesh (Variables|Default|GetSkeletalMesh))
  (bind _returnvalue (Transformation|GetSocketTransform _skeletalmesh "TraceSocket" "RTS_World"))
  (bind (_location _rotation) (Math|Transform|BreakTransform _returnvalue))
  ;[1 1 1] Do Damage on Overlap based on min and max velocties
  (bind _returnvalue_2 (Physics|GetPhysicsLinearVelocity (Variables|Default|GetHitBox) "None"))
  (bind _output_get (Variables|DoNotTouch|SetVelocityDamage (Math|Vector|VectorLength _returnvalue_2)))
  (if (> _output_get (Variables|MeleeWeaponSetup|GetMinimumSwingSpeed))
    (Variables|DoNotTouch|SetVelocityMod (/ (Math|Float|Min(Float) (Variables|DoNotTouch|GetVelocityDamage) _maximumswingspeed) _maximumswingspeed))
    (bind _outhit (Collision|SphereTraceByChannel _location (+ _location (* (Math|Vector|GetRightVector _rotation) (Variables|MeleeWeaponSetup|GetTraceLength))) 3.0 "TraceTypeQuery3" false (Utilities|Array|MakeArray (Variables|Default|GetParent)) "None"))
    (bind _damage (CallFunction|DoHit _outhit))
    (Game|Damage|ApplyPointDamage OtherActor _damage _returnvalue_2 _outhit (Pawn|GetController (Variables|Default|GetParent)) self (Variables|MeleeWeaponSetup|GetDamageType))))

(event EventTriggeron
  ;[1 1 1] Trigger Hold Position Swapping
  (if (and (Variables|MeleeWeaponSetup|GetbUseSecondaryHold) (Variables|DoNotTouch|GetbCanSwap))
    (CallFunction|SwapHoldType)))

(event EventTick
  (params (DeltaSeconds :type Float%20%28single-precision%29))
  (bind _skeletalmesh (Variables|Default|GetSkeletalMesh))
  (bind _skeletalmesh_2 (Variables|Default|GetSkeletalMesh))
  ;[1 1 1] Event Tick
  (Variables|DoNotTouch|SetDeltaSeconds DeltaSeconds)
  (if (and (not (Variables|DoNotTouch|GetbCanSwap)) (Variables|MeleeWeaponSetup|GetbUseSecondaryHold))
    (if (Variables|DoNotTouch|GetbSecondaryHold)
      ;;[0 0 0] Are We Close Enough?
      (if (Class|KismetMathLibrary|NearlyEqualTransformTransform (Transformation|GetRelativeTransform (Variables|Default|GetSkeletalMesh)) (Variables|MeleeWeaponSetup|GetSecondaryHoldTransform) 0.01 0.01 0.01)
        (Variables|DoNotTouch|SetbCanSwap true)
        (else
          ;;[0 0 0] Set location and rotation over time
          (Transformation|SetRelativeTransform _skeletalmesh (Class|KismetMathLibrary|TInterpto (Transformation|GetRelativeTransform _skeletalmesh) (Variables|MeleeWeaponSetup|GetSecondaryHoldTransform) (Variables|DoNotTouch|GetDeltaSeconds) 6.0) false false)))
      (else
        ;;[0 0 0] Are We Close Enough?
        (if (Class|KismetMathLibrary|NearlyEqualTransformTransform (Transformation|GetRelativeTransform (Variables|Default|GetSkeletalMesh)) (Math|Transform|MakeTransform (Variables|Default|GetHeldLocationAdjustment) (Variables|Default|GetHeldRotationAdjustment)) 0.01 0.01 0.01)
          (Variables|DoNotTouch|SetbCanSwap true)
          (else
            ;;[0 0 0] Set Location and Rotation
            (Transformation|SetRelativeTransform _skeletalmesh_2 (Class|KismetMathLibrary|TInterpto (Transformation|GetRelativeTransform _skeletalmesh_2) (Math|Transform|MakeTransform (Variables|Default|GetHeldLocationAdjustment) (Variables|Default|GetHeldRotationAdjustment)) (Variables|DoNotTouch|GetDeltaSeconds) 6.0) false false)))))))

(event EventReleaseObject
  ;[1 1 1] Release
  (|CallParentFunction)
  (Variables|DoNotTouch|SetbAttachedToHand false)
  (Actor|Tick|SetActorTickEnabled false)
  (Variables|DoNotTouch|SetbCanSwap true)
  (Variables|DoNotTouch|SetbSecondaryHold false))

(event EventGrab
  (params (Parent :type BP%20VR%20Character%20Object%20Reference) (Hand :type BP%20VR%20Character%20Hand%20Object%20Reference) (AttachPoint :type Scene%20Component%20Object%20Reference))
  ;[1 1 1] Grab
  (if (not (Variables|Default|GetbHolstered))
    (Utilities|IsValid (Variables|Default|GetParent)
      (:Is%20Not%20Valid
        (|CallParentFunction Parent Hand AttachPoint)
        (Variables|DoNotTouch|SetbAttachedToHand true)
        (Actor|Tick|SetActorTickEnabled true)
        (Variables|DoNotTouch|SetbSecondaryHold false)))))

(event EventHolster
  (params (HolsterComponent :type Skeletal%20Mesh%20Component%20Object%20Reference) (AttachPoint :type Scene%20Component%20Object%20Reference))
  ;[1 1 1] Holster
  (CallFunction|ReleaseObject)
  (CallFunction|AttachtoHolster HolsterComponent AttachPoint)
  (Actor|Tick|SetActorTickEnabled false)
  (Variables|Default|SetbHolstered true)
  (Variables|DoNotTouch|SetbCanSwap true)
  (Variables|DoNotTouch|SetbSecondaryHold false))

(event EventUnHolster
  (params (Parent :type BP%20VR%20Character%20Object%20Reference) (Hand :type BP%20VR%20Character%20Hand%20Object%20Reference) (AttachPoint :type Scene%20Component%20Object%20Reference))
  ;[1 1 1] Unholster
  (CallFunction|DetachfromHolster)
  (CallFunction|Grab Parent Hand AttachPoint)
  (Actor|Tick|SetActorTickEnabled true))

(event EventBeginPlay
  (bind _skeletalmesh (Variables|Default|GetSkeletalMesh))
  ;[1 1 1] Begin play
  (Variables|DoNotTouch|SetbCanSwap true)
  ;;[0 0 0] Turn physics off if we have a parent,  on if we do not.
  (Utilities|IsValid (Variables|Default|GetParent)
    (:Is%20Valid
      (Physics|SetSimulatePhysics _skeletalmesh false)
      (Actor|Tick|SetActorTickEnabled true))
    (:Is%20Not%20Valid
      (Physics|SetSimulatePhysics _skeletalmesh true)
      (Actor|Tick|SetActorTickEnabled false))))

(fn ConstructionScript
  (|CallParentFunction)
  ;[1 1 1] Attach components to correct socket
  (Transformation|AttachComponentToComponent (Variables|Default|GetHitBox) (Variables|Default|GetSkeletalMesh) "BladeSocket" "SnapToTarget" "SnapToTarget" "KeepWorld" true))

(fn DoHit
  (params (Hit :type Hit%20Result%20Structure))
  (bind (_bblockinghit _binitialoverlap _time _location _impactpoint _normal _impactnormal _physmat _hitactor _hitcomponent) (Collision|BreakHitResult Hit))
  (bind _fleshhitsound (Variables|MeleeWeaponHitSounds|GetFleshHitSound))
  (bind _woodhitsound (Variables|MeleeWeaponHitSounds|GetWoodHitSound))
  (bind _concretehitsound (Variables|MeleeWeaponHitSounds|GetConcreteHitSound))
  (bind _plasterhitsound (Variables|MeleeWeaponHitSounds|GetPlasterHitSound))
  (bind _metalhitsound (Variables|MeleeWeaponHitSounds|GetMetalHitSound))
  (bind _groundhitsound (Variables|MeleeWeaponHitSounds|GetGroundHitSound))
  (bind _fleshhitsound_2 (Variables|MeleeWeaponHitSounds|GetFleshHitSound))
  (bind _defaulteffects (Variables|MeleeWeaponEffects|GetDefaultEffects))
  (bind _defaultdecals (Variables|MeleeWeaponDecals|GetDefaultDecals))
  (bind _defaulthitsound (Variables|MeleeWeaponHitSounds|GetDefaultHitSound))
  (bind _flesheffects (Variables|MeleeWeaponEffects|GetFleshEffects))
  (bind _wooddecals (Variables|MeleeWeaponDecals|GetWoodDecals))
  (bind _woodeffects (Variables|MeleeWeaponEffects|GetWoodEffects))
  (bind _concretedecals (Variables|MeleeWeaponDecals|GetConcreteDecals))
  (bind _concreteeffects (Variables|MeleeWeaponEffects|GetConcreteEffects))
  (bind _plasterdecals (Variables|MeleeWeaponDecals|GetPlasterDecals))
  (bind _plastereffects (Variables|MeleeWeaponEffects|GetPlasterEffects))
  (bind _metaldecals (Variables|MeleeWeaponDecals|GetMetalDecals))
  (bind _metaleffects (Variables|MeleeWeaponEffects|GetMetalEffects))
  (bind _groundeffects (Variables|MeleeWeaponEffects|GetGroundEffects))
  (bind _grounddecals (Variables|MeleeWeaponDecals|GetGroundDecals))
  (bind _flesheffects_2 (Variables|MeleeWeaponEffects|GetFleshEffects))
  (bind _returnvalue (Math|Rotator|MakeRotfromX _impactnormal))
  ;[1 1 1] Trace for hit and then set decal, effect, and sound
  (if _bblockinghit
    (LocalVariables|SetTempComponent _hitcomponent)
    (switch Utilities|FlowControl|Switch|SwitchonEPhysicalSurface (Variables|/Script/Engine.PhysicalMaterial|GetSurfaceType _physmat)
      (:SurfaceType_Default
        (if (> (Utilities|Array|Length (Variables|MeleeWeaponDecals|GetDefaultDecals)) 0)
          (LocalVariables|SetDecalMaterial (Utilities|Array|Get(acopy) _defaultdecals (Math|Random|RandomInteger (Utilities|Array|Length _defaultdecals)))))
        (if (> (Utilities|Array|Length (Variables|MeleeWeaponEffects|GetDefaultEffects)) 0)
          (LocalVariables|SetImpactEffect (Utilities|Array|Get(acopy) _defaulteffects (Math|Random|RandomInteger (Utilities|Array|Length _defaulteffects)))))
        (if (> (Utilities|Array|Length (Variables|MeleeWeaponHitSounds|GetDefaultHitSound)) 0)
          (LocalVariables|SetImpactSound (Utilities|Array|Get(acopy) _defaulthitsound (Math|Random|RandomInteger (Utilities|Array|Length _defaulthitsound))))))
      (:SurfaceType1
        (LocalVariables|SetTempDamage (* (Variables|MeleeWeaponSetup|GetDamage) (Variables|DoNotTouch|GetVelocityMod)) :!label _label)
        (if (> (Utilities|Array|Length (Variables|MeleeWeaponEffects|GetFleshEffects)) 0)
          (LocalVariables|SetImpactEffect (Utilities|Array|Get(acopy) _flesheffects_2 (Math|Random|RandomInteger (Utilities|Array|Length _flesheffects_2)))))
        (if (> (Utilities|Array|Length (Variables|MeleeWeaponHitSounds|GetFleshHitSound)) 0)
          (LocalVariables|SetImpactSound (Utilities|Array|Get(acopy) _fleshhitsound (Math|Random|RandomInteger (Utilities|Array|Length _fleshhitsound))))))
      (:SurfaceType2
        (if (> (Utilities|Array|Length (Variables|MeleeWeaponDecals|GetWoodDecals)) 0)
          (LocalVariables|SetDecalMaterial (Utilities|Array|Get(acopy) _wooddecals (Math|Random|RandomInteger (Utilities|Array|Length _wooddecals)))))
        (if (> (Utilities|Array|Length (Variables|MeleeWeaponEffects|GetWoodEffects)) 0)
          (LocalVariables|SetImpactEffect (Utilities|Array|Get(acopy) _woodeffects (Math|Random|RandomInteger (Utilities|Array|Length _woodeffects)))))
        (if (> (Utilities|Array|Length (Variables|MeleeWeaponHitSounds|GetWoodHitSound)) 0)
          (LocalVariables|SetImpactSound (Utilities|Array|Get(acopy) _woodhitsound (Math|Random|RandomInteger (Utilities|Array|Length _woodhitsound))))))
      (:SurfaceType3
        (if (> (Utilities|Array|Length (Variables|MeleeWeaponDecals|GetConcreteDecals)) 0) :!label _label_2
          (LocalVariables|SetDecalMaterial (Utilities|Array|Get(acopy) _concretedecals (Math|Random|RandomInteger (Utilities|Array|Length _concretedecals)))))
        (if (> (Utilities|Array|Length (Variables|MeleeWeaponEffects|GetConcreteEffects)) 0)
          (LocalVariables|SetImpactEffect (Utilities|Array|Get(acopy) _concreteeffects (Math|Random|RandomInteger (Utilities|Array|Length _concreteeffects)))))
        (if (> (Utilities|Array|Length (Variables|MeleeWeaponHitSounds|GetConcreteHitSound)) 0)
          (LocalVariables|SetImpactSound (Utilities|Array|Get(acopy) _concretehitsound (Math|Random|RandomInteger (Utilities|Array|Length _concretehitsound))))))
      (:SurfaceType4
        (if (> (Utilities|Array|Length (Variables|MeleeWeaponDecals|GetPlasterDecals)) 0)
          (LocalVariables|SetDecalMaterial (Utilities|Array|Get(acopy) _plasterdecals (Math|Random|RandomInteger (Utilities|Array|Length _plasterdecals)))))
        (if (> (Utilities|Array|Length (Variables|MeleeWeaponEffects|GetPlasterEffects)) 0)
          (LocalVariables|SetImpactEffect (Utilities|Array|Get(acopy) _plastereffects (Math|Random|RandomInteger (Utilities|Array|Length _plastereffects)))))
        (if (> (Utilities|Array|Length (Variables|MeleeWeaponHitSounds|GetPlasterHitSound)) 0)
          (LocalVariables|SetImpactSound (Utilities|Array|Get(acopy) _plasterhitsound (Math|Random|RandomInteger (Utilities|Array|Length _plasterhitsound))))))
      (:SurfaceType5
        (if (> (Utilities|Array|Length (Variables|MeleeWeaponDecals|GetMetalDecals)) 0)
          (LocalVariables|SetDecalMaterial (Utilities|Array|Get(acopy) _metaldecals (Math|Random|RandomInteger (Utilities|Array|Length _metaldecals)))))
        (if (> (Utilities|Array|Length (Variables|MeleeWeaponEffects|GetMetalEffects)) 0)
          (LocalVariables|SetImpactEffect (Utilities|Array|Get(acopy) _metaleffects (Math|Random|RandomInteger (Utilities|Array|Length _metaleffects)))))
        (if (> (Utilities|Array|Length (Variables|MeleeWeaponHitSounds|GetMetalHitSound)) 0)
          (LocalVariables|SetImpactSound (Utilities|Array|Get(acopy) _metalhitsound (Math|Random|RandomInteger (Utilities|Array|Length _metalhitsound))))))
      (:SurfaceType6
        (if (> (Utilities|Array|Length (Variables|MeleeWeaponDecals|GetGroundDecals)) 0) :!label _label_3
          (LocalVariables|SetDecalMaterial (Utilities|Array|Get(acopy) _grounddecals (Math|Random|RandomInteger (Utilities|Array|Length _grounddecals)))))
        (if (> (Utilities|Array|Length (Variables|MeleeWeaponEffects|GetGroundEffects)) 0)
          (LocalVariables|SetImpactEffect (Utilities|Array|Get(acopy) _groundeffects (Math|Random|RandomInteger (Utilities|Array|Length _groundeffects)))))
        (if (> (Utilities|Array|Length (Variables|MeleeWeaponHitSounds|GetGroundHitSound)) 0)
          (LocalVariables|SetImpactSound (Utilities|Array|Get(acopy) _groundhitsound (Math|Random|RandomInteger (Utilities|Array|Length _groundhitsound))))))
      (:SurfaceType7
        (LocalVariables|SetTempDamage (* (* (Variables|MeleeWeaponSetup|GetDamage) (Variables|DoNotTouch|GetVelocityMod)) (Variables|MeleeWeaponSetup|GetCriticalMultiplier)))
        (if (> (Utilities|Array|Length (Variables|MeleeWeaponEffects|GetFleshEffects)) 0)
          (LocalVariables|SetImpactEffect (Utilities|Array|Get(acopy) _flesheffects (Math|Random|RandomInteger (Utilities|Array|Length _flesheffects)))))
        (if (> (Utilities|Array|Length (Variables|MeleeWeaponHitSounds|GetFleshHitSound)) 0)
          (LocalVariables|SetImpactSound (Utilities|Array|Get(acopy) _fleshhitsound_2 (Math|Random|RandomInteger (Utilities|Array|Length _fleshhitsound_2))))))
      (:SurfaceType8
        (goto _label_2))
      (:SurfaceType9
        (goto _label))
      (:SurfaceType10
        (goto _label_3)))
    ;[1 1 1] Do Impact Logic Here
    (if (Utilities|IsValidClass (LocalVariables|GetDecalMaterial))
      (if (or (Utilities|Enum|Equal(Enum) (Collision|GetCollisionObjectType (LocalVariables|GetTempComponent)) "ECC_WorldStatic") (Utilities|Enum|Equal(Enum) (Collision|GetCollisionObjectType (LocalVariables|GetTempComponent)) "ECC_GameTraceChannel17"))
        (bind _returnvalue_2 (Game|SpawnActorfromClass (LocalVariables|GetDecalMaterial) (Math|Transform|MakeTransform _location _returnvalue) "AlwaysSpawn" 0 0))
        (Transformation|SetActorRotation _returnvalue_2 _returnvalue)))
    (Utilities|IsValid (LocalVariables|GetImpactEffect)
      (:Is%20Valid
        (Effects|SpawnEmitteratLocation (LocalVariables|GetImpactEffect) _location _returnvalue))
      (:Is%20Not%20Valid
        _))
    (Utilities|IsValid (LocalVariables|GetImpactSound)
      (:Is%20Valid
        (Audio|PlaySoundatLocation (LocalVariables|GetImpactSound) _location))
      (:Is%20Not%20Valid
        _))
    (return (Math|Conversions|ToFloat(Integer) (Math|Float|Round (LocalVariables|GetTempDamage))))
    (else
      (return 0.0))))

(fn AttachtoHolster
  (params (HolsterComponent :type Skeletal%20Mesh%20Component%20Object%20Reference) (AttachPoint :type Scene%20Component%20Object%20Reference))
  ;[1 1 1] Attach to Holster
  (Utilities|IsValid HolsterComponent
    (:Is%20Valid
      (Utilities|IsValid AttachPoint
        (:Is%20Valid
          ;;[0 0 0] SetHolsterParent
          (Variables|Default|SetHolsterParent HolsterComponent)
          (bind _output_get (Variables|Default|SetAttachPoint AttachPoint))
          ;;[0 0 0] Turn off Physics
          (Physics|SetSimulatePhysics (Variables|Default|GetSkeletalMesh) false)
          ;;[0 0 0] Turn off Overlap Events so we cannot grab
          (Variables|/Script/Engine.PrimitiveComponent|SetbGenerateOverlapEvents (Variables|Default|GetSkeletalMesh) false)
          ;;[0 0 0] Attach to Holster and set location and rotation adjustments
          (Transformation|AttachComponentToComponent (Variables|Default|GetRoot) _output_get "None" "SnapToTarget" "SnapToTarget" "KeepWorld" false)
          (Transformation|AttachComponentToComponent (Variables|Default|GetSkeletalMesh) (Variables|Default|GetRoot) "None" "SnapToTarget" "SnapToTarget" "KeepWorld" false)
          (Transformation|SetRelativeLocationAndRotation (Variables|Default|GetSkeletalMesh) (Variables|Default|GetHolsterLocationAdjustment) (Variables|Default|GetHolsterRotationAdjustment) false false)
          ;;[0 0 0] Play Sound
          (Audio|PlaySoundatLocation (Variables|MeleeWeaponSounds|GetHolsterSound) (Transformation|GetWorldLocation (Variables|Default|GetSkeletalMesh)))
          ;;[0 0 0] Clear Varaible
          (Variables|Default|SetParentHand 0))))))

(fn DetachfromHolster
  ;[1 1 1] Detach from holster and clear variables
  (Transformation|DetachFromComponent (Variables|Default|GetRoot) "KeepWorld" "KeepWorld" "KeepWorld" false)
  ;;[0 0 0] Turn on overlap events so we can grab again
  (Variables|/Script/Engine.PrimitiveComponent|SetbGenerateOverlapEvents (Variables|Default|GetSkeletalMesh) true)
  (Variables|Default|SetHolsterParent 0)
  (Variables|Default|SetAttachPoint 0)
  (Variables|Default|SetbHolstered false))

(fn SwapHoldType
  (if (Variables|DoNotTouch|GetbSecondaryHold)
    (Variables|DoNotTouch|SetbSecondaryHold false)
    (else
      (Variables|DoNotTouch|SetbSecondaryHold true)))
  (Variables|DoNotTouch|SetbCanSwap false))