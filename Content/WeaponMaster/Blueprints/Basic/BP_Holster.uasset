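; VR holster slot that stores one interaction object of a matching HolsterType and returns it to a hand.
; Trigger overlap registers a single hand, then CanHolster or CanUnholster sets the permission flag and material "State" highlight.
; Holster and Unholster act on those flags.
; Outside arcade mode, firearms require the main hand, or dynamic main-hand switching with the opposite hand empty; other types are grabbed by either hand.
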(event OnComponentBeginOverlap(Trigger)
  (params (OverlappedComponent :type Primitive%20Component%20Object%20Reference) (OtherActor :type Actor%20Object%20Reference) (OtherComp :type Primitive%20Component%20Object%20Reference) (OtherBodyIndex :type Integer) (bFromSweep :type Boolean) (SweepResult :type Hit%20Result%20Structure%20%28by%20ref%29))
  (Utilities|IsValid (Variables|DoNotTouch|GetCurrentHand)
    (:Is%20Not%20Valid
      (bind _asbp_vrcharacter_hand (Utilities|Casting|CastToBP_VRCharacterHand OtherActor))
      (bind _output_get (Variables|DoNotTouch|SetCurrentHand _asbp_vrcharacter_hand))
      (Variables|/Game/WeaponMaster/Blueprints/Basic/BP_VRCharacterHand.BP_VRCharacterHand_C|SetCurrentHolsterObject _output_get self)
      (Utilities|IsValid (Variables|DoNotTouch|GetCurrentObject)
        (:Is%20Valid
          (CallFunction|CanUnholster))
        (:Is%20Not%20Valid
          (CallFunction|CanHolster))))))

(event OnComponentEndOverlap(Trigger)
  (params (OverlappedComponent :type Primitive%20Component%20Object%20Reference) (OtherActor :type Actor%20Object%20Reference) (OtherComp :type Primitive%20Component%20Object%20Reference) (OtherBodyIndex :type Integer))
  (if (== OtherActor (Variables|DoNotTouch|GetCurrentHand))
    (Variables|DoNotTouch|SetbCanUnholster false)
    (Variables|DoNotTouch|SetbCanHolster false)
    (Variables|/Game/WeaponMaster/Blueprints/Basic/BP_VRCharacterHand.BP_VRCharacterHand_C|SetCurrentHolsterObject (Variables|DoNotTouch|GetCurrentHand) 0)
    (Variables|DoNotTouch|SetCurrentHand 0)
    (Rendering|Material|SetScalarParameterValueonMaterials (Variables|Default|GetMesh) "State" 0.0)))

(event EventBeginPlay)

(event Collision|EventActorBeginOverlap
  (params (OtherActor :type Actor%20Object%20Reference)))

(event EventTick
  (params (DeltaSeconds :type Float%20%28single-precision%29)))

(fn ConstructionScript)

(fn CanHolster
  (bind _currenthand (Variables|DoNotTouch|GetCurrentHand))
  (bind _attachedactor (Variables|/Game/WeaponMaster/VirtualRealityBP/Blueprints/BP_MotionController.BP_MotionController_C|GetAttachedActor _currenthand))
  (Utilities|IsValid _attachedactor
    (:Is%20Valid
      (bind _asbp_interaction_object (Utilities|Casting|CastToBP_InteractionObject _attachedactor)
        (:then
          (if (Utilities|Enum|Equal(Enum) (Variables|/Game/WeaponMaster/Blueprints/Basic/BP_InteractionObject.BP_InteractionObject_C|GetHolsterType _asbp_interaction_object) (Variables|HolsterSetup|GetHolsterType))
            (Rendering|Material|SetScalarParameterValueonMaterials (Variables|Default|GetMesh) "State" 1.0)
            (Variables|DoNotTouch|SetbCanHolster true)
            (else
              (Rendering|Material|SetScalarParameterValueonMaterials (Variables|Default|GetMesh) "State" 0.0)
              (Variables|DoNotTouch|SetbCanHolster false))))
        (:CastFailed
          (Rendering|Material|SetScalarParameterValueonMaterials (Variables|Default|GetMesh) "State" 0.0 :!label _label)
          (Variables|DoNotTouch|SetbCanHolster false))))
    (:Is%20Not%20Valid
      (goto _label))))

(fn CanUnholster
  (Utilities|IsValid (Variables|/Game/WeaponMaster/VirtualRealityBP/Blueprints/BP_MotionController.BP_MotionController_C|GetAttachedActor (Variables|DoNotTouch|GetCurrentHand))
    (:Is%20Valid
      (Rendering|Material|SetScalarParameterValueonMaterials (Variables|Default|GetMesh) "State" 0.0)
      (Variables|DoNotTouch|SetbCanUnholster false))
    (:Is%20Not%20Valid
      (switch Utilities|FlowControl|Switch|SwitchonEnum_ObjectTypes (Variables|/Game/WeaponMaster/Blueprints/Basic/BP_InteractionObject.BP_InteractionObject_C|GetObjectType (Variables|DoNotTouch|GetCurrentObject))
        (:NewEnumerator0
          (if (not (Variables|/Game/WeaponMaster/Blueprints/Basic/BP_VRCharacter.BP_VRCharacter_C|GetArcadeMode (Variables|DoNotTouch|GetParent))) :!label _label
            (if (Variables|/Game/WeaponMaster/Blueprints/Basic/BP_VRCharacterHand.BP_VRCharacterHand_C|GetbIsMainHand (Variables|DoNotTouch|GetCurrentHand))
              (Rendering|Material|SetScalarParameterValueonMaterials (Variables|Default|GetMesh) "State" 1.0)
              (Variables|DoNotTouch|SetbCanUnholster true)
              (else
                ;[1 1 1] Are we using dynamic main hand
                (if (Variables|/Game/WeaponMaster/Blueprints/Basic/BP_VRCharacter.BP_VRCharacter_C|GetbUseDynamicMainHand (Variables|DoNotTouch|GetParent))
                  ;[0 0 0] What Hand are we?
                  (switch Utilities|FlowControl|Switch|SwitchonEControllerHand (Variables|/Game/WeaponMaster/VirtualRealityBP/Blueprints/BP_MotionController.BP_MotionController_C|GetHand (Variables|DoNotTouch|GetCurrentHand))
                    (:Left
                      ;[0 0 0] Is there an object in the opposite hand?
                      (Utilities|IsValid (Variables|/Game/WeaponMaster/VirtualRealityBP/Blueprints/BP_MotionController.BP_MotionController_C|GetAttachedActor (Variables|/Game/WeaponMaster/Blueprints/Basic/BP_VRCharacter.BP_VRCharacter_C|GetRightHand (Variables|DoNotTouch|GetParent)))
                        (:Is%20Not%20Valid
                          _)))
                    (:Right
                      ;[0 0 0] Is there an object in the opposite hand?
                      (Utilities|IsValid (Variables|/Game/WeaponMaster/VirtualRealityBP/Blueprints/BP_MotionController.BP_MotionController_C|GetAttachedActor (Variables|/Game/WeaponMaster/Blueprints/Basic/BP_VRCharacter.BP_VRCharacter_C|GetLeftHand (Variables|DoNotTouch|GetParent)))
                        (:Is%20Not%20Valid
                          _))))
                  (Rendering|Material|SetScalarParameterValueonMaterials (Variables|Default|GetMesh) "State" 1.0)
                  (Variables|DoNotTouch|SetbCanUnholster true)
                  (else
                    (Rendering|Material|SetScalarParameterValueonMaterials (Variables|Default|GetMesh) "State" 0.0)
                    (Variables|DoNotTouch|SetbCanUnholster false)))))
            (else
              (Rendering|Material|SetScalarParameterValueonMaterials (Variables|Default|GetMesh) "State" 1.0 :!label _label_2)
              (Variables|DoNotTouch|SetbCanUnholster true))))
        (:NewEnumerator1
          (goto _label))
        (:NewEnumerator5
          (goto _label_2))
        (:NewEnumerator6
          (goto _label_2))
        (:NewEnumerator8
          (goto _label_2))
        (:NewEnumerator7
          (goto _label_2))))))

(fn SetParent)

(fn Unholster
  (bind _currenthand (Variables|DoNotTouch|GetCurrentHand))
  (bind _currenthand_2 (Variables|DoNotTouch|GetCurrentHand))
  (bind _currenthand_3 (Variables|DoNotTouch|GetCurrentHand))
  (bind _currenthand_4 (Variables|DoNotTouch|GetCurrentHand))
  (if (Variables|DoNotTouch|GetbCanUnholster)
    (switch Utilities|FlowControl|Switch|SwitchonEnum_ObjectTypes (Variables|/Game/WeaponMaster/Blueprints/Basic/BP_InteractionObject.BP_InteractionObject_C|GetObjectType (Variables|DoNotTouch|GetCurrentObject))
      (:NewEnumerator0
        (if (not (Variables|/Game/WeaponMaster/Blueprints/Basic/BP_VRCharacter.BP_VRCharacter_C|GetArcadeMode (Variables|DoNotTouch|GetParent))) :!label _label
          _
          (else
            (Default|Grab (Variables|DoNotTouch|GetCurrentObject) (Variables|DoNotTouch|GetParent) _currenthand_4 (Variables|/Game/WeaponMaster/Blueprints/Basic/BP_VRCharacterHand.BP_VRCharacterHand_C|GetAttachPoint _currenthand_4) :!label _label_2)
            (Variables|DoNotTouch|SetCurrentObject 0)
            (Variables|DoNotTouch|SetbCanUnholster false)
            (CallFunction|CanHolster)
            (return 0))))
      (:NewEnumerator1
        (goto _label))
      (:NewEnumerator5
        (goto _label_2))
      (:NewEnumerator6
        (goto _label_2))
      (:NewEnumerator8
        (goto _label_2))
      (:NewEnumerator7
        (goto _label_2)))
    (if (Variables|/Game/WeaponMaster/Blueprints/Basic/BP_VRCharacterHand.BP_VRCharacterHand_C|GetbIsMainHand (Variables|DoNotTouch|GetCurrentHand))
      (Default|UnHolster (Variables|DoNotTouch|GetCurrentObject) (Variables|DoNotTouch|GetParent) _currenthand (Variables|/Game/WeaponMaster/Blueprints/Basic/BP_VRCharacterHand.BP_VRCharacterHand_C|GetAttachPoint _currenthand))
      (Variables|DoNotTouch|SetCurrentObject 0)
      (Variables|DoNotTouch|SetbCanUnholster false)
      (CallFunction|CanHolster)
      (return 0)
      (else
        ;[1 1 1] Are we using dynamic main hand
        (if (Variables|/Game/WeaponMaster/Blueprints/Basic/BP_VRCharacter.BP_VRCharacter_C|GetbUseDynamicMainHand (Variables|DoNotTouch|GetParent))
          ;[0 0 0] What Hand are we?
          (switch Utilities|FlowControl|Switch|SwitchonEControllerHand (Variables|/Game/WeaponMaster/VirtualRealityBP/Blueprints/BP_MotionController.BP_MotionController_C|GetHand (Variables|DoNotTouch|GetCurrentHand))
            (:Left
              ;[0 0 0] Is there an object in the opposite hand?
              (Utilities|IsValid (Variables|/Game/WeaponMaster/VirtualRealityBP/Blueprints/BP_MotionController.BP_MotionController_C|GetAttachedActor (Variables|/Game/WeaponMaster/Blueprints/Basic/BP_VRCharacter.BP_VRCharacter_C|GetRightHand (Variables|DoNotTouch|GetParent)))
                (:Is%20Not%20Valid
                  ;[0 0 0] Set new main hand
                  (Default|SetMainHand (Variables|DoNotTouch|GetParent) "Left")
                  ;[0 0 0] Grab
                  (Default|UnHolster (Variables|DoNotTouch|GetCurrentObject) (Variables|DoNotTouch|GetParent) _currenthand_3 (Variables|/Game/WeaponMaster/Blueprints/Basic/BP_VRCharacterHand.BP_VRCharacterHand_C|GetAttachPoint _currenthand_3))
                  (Default|RumbleController (Variables|DoNotTouch|GetCurrentHand) 0.7)
                  (Variables|DoNotTouch|SetCurrentObject 0)
                  (Variables|DoNotTouch|SetbCanUnholster false)
                  (CallFunction|CanHolster)
                  (return 0))))
            (:Right
              ;[0 0 0] Is there an object in the opposite hand?
              (Utilities|IsValid (Variables|/Game/WeaponMaster/VirtualRealityBP/Blueprints/BP_MotionController.BP_MotionController_C|GetAttachedActor (Variables|/Game/WeaponMaster/Blueprints/Basic/BP_VRCharacter.BP_VRCharacter_C|GetLeftHand (Variables|DoNotTouch|GetParent)))
                (:Is%20Not%20Valid
                  ;[0 0 0] Set new main hand
                  (Default|SetMainHand (Variables|DoNotTouch|GetParent) "Right")
                  ;[0 0 0] Grab
                  (Default|UnHolster (Variables|DoNotTouch|GetCurrentObject) (Variables|DoNotTouch|GetParent) _currenthand_2 (Variables|/Game/WeaponMaster/Blueprints/Basic/BP_VRCharacterHand.BP_VRCharacterHand_C|GetAttachPoint _currenthand_2))
                  (Default|RumbleController (Variables|DoNotTouch|GetCurrentHand) 0.7)
                  (Variables|DoNotTouch|SetCurrentObject 0)
                  (Variables|DoNotTouch|SetbCanUnholster false)
                  (CallFunction|CanHolster)
                  (return 0))))))))))

(fn Holster
  (if (Variables|DoNotTouch|GetbCanHolster)
    (bind _asbp_interaction_object (Utilities|Casting|CastToBP_InteractionObject (Variables|/Game/WeaponMaster/VirtualRealityBP/Blueprints/BP_MotionController.BP_MotionController_C|GetAttachedActor (Variables|DoNotTouch|GetCurrentHand))))
    (Default|Holster _asbp_interaction_object (Variables|Default|GetMesh) (Variables|Default|GetAttachPoint))
    (Variables|DoNotTouch|SetCurrentObject _asbp_interaction_object)))