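; Base Blueprint for hand-held weapon attachments such as scopes, grips and muzzles, extended by children through attach and detach events.
; Grabbing it shows matching attachment zones on a firearm in the opposite hand; releasing it hides them.
; Detaching from a held advanced or simple firearm requires the weapon's permission, clears its slot, updates stats on advanced firearms only, and passes the attachment to the grabbing hand.
; A short timer then re-enables attaching.
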(event Custom|DetachGrab
  (params (Parent :type BP%20VR%20Character%20Object%20Reference) (Hand%20 :type BP%20VR%20Character%20Hand%20Object%20Reference) (AttachPoint :type Scene%20Component%20Object%20Reference))
  ;[1 1 1] When we detach we need to do a seperate grab to add to hand
  (|CallParentFunction Parent Hand%20 AttachPoint)
  ;[1 1 1] Call to parent grab and set variables before calling attachedtohand
  (Variables|DoNotTouch|SetbAttachedToHand true)
  (CallFunction|AttachedtoHand))

(event Custom|StartResetTimer
  ;[1 1 1] Timer for how soon we can reattach to weapon.
  (Utilities|Time|SetTimerbyEvent (delegate Custom|ResetCanAttach) 0.5))

(event Custom|ResetCanAttach
  ;[1 1 1] Timer for how soon we can reattach to weapon.
  (Variables|DoNotTouch|SetbCanAttach true))

(event Custom|AttachedToHand
  ;[1 1 1] When first attached to hand we need to show the attachments zones on the opposite hands weapon (if available)
  (CallFunction|CheckOppositeHandforWeapon))

(event Custom|AttachedToWeapon
  ;[1 1 1] Overrided, or extended, by children
  (Variables|DoNotTouch|SetbCanAttach false)
  (Collision|SetCollisionEnabled (Variables|Default|GetSkeletalMesh) "QueryOnly"))

(event Custom|DetachedFromWeapon
  ;[1 1 1] Overrided, or extended, by children
)

(event EventBeginPlay
  ;[1 1 1] Begin Play
  ;;[0 0 0] Set simultate physics based on if we start out attached to a weapon or not.
  (Utilities|IsValid (Variables|DoNotTouch|GetWeaponParent)
    (:Is%20Valid
      (Variables|DoNotTouch|SetbCanAttach false))
    (:Is%20Not%20Valid
      (Physics|SetSimulatePhysics (Variables|Default|GetSkeletalMesh) true)
      (Variables|DoNotTouch|SetbCanAttach true))))

(event EventGrab
  (params (Parent :type BP%20VR%20Character%20Object%20Reference) (Hand :type BP%20VR%20Character%20Hand%20Object%20Reference) (AttachPoint :type Scene%20Component%20Object%20Reference))
  ;[1 1 1] Call to parent grab and set variables before calling attachedtohand
  (|CallParentFunction Parent Hand AttachPoint)
  (Variables|DoNotTouch|SetbAttachedToHand true)
  (CallFunction|AttachedtoHand))

(event EventReleaseObject
  (bind _parent (Variables|Default|GetParent))
  (bind _parent_2 (Variables|Default|GetParent))
  (bind _righthand (Variables|/Game/WeaponMaster/Blueprints/Basic/BP_VRCharacter.BP_VRCharacter_C|GetRightHand _parent))
  (bind _lefthand (Variables|/Game/WeaponMaster/Blueprints/Basic/BP_VRCharacter.BP_VRCharacter_C|GetLeftHand _parent_2))
  (bind _attachedactor (Variables|/Game/WeaponMaster/VirtualRealityBP/Blueprints/BP_MotionController.BP_MotionController_C|GetAttachedActor _righthand))
  (bind _attachedactor_2 (Variables|/Game/WeaponMaster/VirtualRealityBP/Blueprints/BP_MotionController.BP_MotionController_C|GetAttachedActor _lefthand))
  ;[1 1 1] Dropping the attachment
  (switch Utilities|FlowControl|Switch|SwitchonEControllerHand (Variables|/Game/WeaponMaster/VirtualRealityBP/Blueprints/BP_MotionController.BP_MotionController_C|GetHand (Variables|Default|GetParentHand))
    (:Left
      (Utilities|IsValid _attachedactor
        (:Is%20Valid
          (bind _asbp_interaction_object (Utilities|Casting|CastToBP_InteractionObject _attachedactor)
            (:then
              (CallFunction|ResetAttachmentZones _asbp_interaction_object)
              (|CallParentFunction :!label _label)
              (Variables|DoNotTouch|SetbAttachedToHand false))
            (:CastFailed
              (Development|PrintString "Not BP_InteractionObject" false :!label _label_2))))
        (:Is%20Not%20Valid
          (goto _label))))
    (:Right
      (Utilities|IsValid _attachedactor_2
        (:Is%20Valid
          (bind _asbp_interaction_object_2 (Utilities|Casting|CastToBP_InteractionObject _attachedactor_2)
            (:then
              (CallFunction|ResetAttachmentZones _asbp_interaction_object_2)
              (goto _label))
            (:CastFailed
              (goto _label_2))))
        (:Is%20Not%20Valid
          (goto _label))))))

(fn ConstructionScript
  ;[1 1 1] Call to parent construction
  (|CallParentFunction))

(fn DetachfromWeapon
  (params (Parent :type BP%20VR%20Character%20Object%20Reference) (ParentHand :type BP%20VR%20Character%20Hand%20Object%20Reference) (AttachPoint :type Scene%20Component%20Object%20Reference))
  ;[1 1 1] If attachment can be removed then we need to detach before reseting the weapons attachment variable for this attachment. Then we attach the attachment to the hand that initiated the detach. Last we call detached from weapon before starting the reset timer.
  (Utilities|IsValid (Variables|/Game/WeaponMaster/Blueprints/Basic/BP_InteractionObject.BP_InteractionObject_C|GetParent (Variables|DoNotTouch|GetWeaponParent))
    (:Is%20Valid
      (bind _canremove (CallFunction|CheckCanRemove))
      (if _canremove
        (Transformation|DetachFromComponent (Variables|Default|GetRoot) "KeepWorld" "KeepWorld" "KeepWorld" true)
        (Variables|DoNotTouch|SetbAttachedToWeapon false)
        (switch Utilities|FlowControl|Switch|SwitchonEnum_ObjectTypes (Variables|/Game/WeaponMaster/Blueprints/Basic/BP_InteractionObject.BP_InteractionObject_C|GetObjectType (Variables|DoNotTouch|GetWeaponParent))
          (:NewEnumerator0
            (bind _asbp_advanced_firearm (Utilities|Casting|CastToBP_AdvancedFirearm (Variables|DoNotTouch|GetWeaponParent))
              (:then
                (switch Utilities|FlowControl|Switch|SwitchonEnum_AttachmentTypes (Variables|AttachmentSetup|GetAttachmentType)
                  (:NewEnumerator0
                    (Variables|/Game/WeaponMaster/Blueprints/Basic/BP_AdvancedFirearm.BP_AdvancedFirearm_C|SetCurrentScopeAttachment _asbp_advanced_firearm 0))
                  (:NewEnumerator1
                    (Variables|/Game/WeaponMaster/Blueprints/Basic/BP_AdvancedFirearm.BP_AdvancedFirearm_C|SetCurrentSideAttachment _asbp_advanced_firearm 0))
                  (:NewEnumerator2
                    (Variables|/Game/WeaponMaster/Blueprints/Basic/BP_AdvancedFirearm.BP_AdvancedFirearm_C|SetCurrentIronsightAttachment _asbp_advanced_firearm 0))
                  (:NewEnumerator4
                    (Variables|/Game/WeaponMaster/Blueprints/Basic/BP_AdvancedFirearm.BP_AdvancedFirearm_C|SetCurrentGripAttachment _asbp_advanced_firearm 0))
                  (:NewEnumerator5
                    (Variables|/Game/WeaponMaster/Blueprints/Basic/BP_AdvancedFirearm.BP_AdvancedFirearm_C|SetCurrentMuzzleAttachment _asbp_advanced_firearm 0)))
                (Default|UpdateWeaponStats _asbp_advanced_firearm)
                (Variables|DoNotTouch|SetWeaponParent 0)
                (CallFunction|DetachGrab Parent ParentHand AttachPoint :!label _label)
                (CallFunction|DetachedfromWeapon)
                (CallFunction|StartResetTimer))
              (:CastFailed
                (Development|PrintString "Not PhysMagWeap" false))))
          (:NewEnumerator1
            (bind _asbp_simple_firearm (Utilities|Casting|CastToBP_SimpleFirearm (Variables|DoNotTouch|GetWeaponParent))
              (:then
                (switch Utilities|FlowControl|Switch|SwitchonEnum_AttachmentTypes (Variables|AttachmentSetup|GetAttachmentType)
                  (:NewEnumerator0
                    (Variables|/Game/WeaponMaster/Blueprints/Basic/BP_SimpleFirearm.BP_SimpleFirearm_C|SetCurrentScopeAttachment _asbp_simple_firearm 0))
                  (:NewEnumerator1
                    (Variables|/Game/WeaponMaster/Blueprints/Basic/BP_SimpleFirearm.BP_SimpleFirearm_C|SetCurrentSideAttachment _asbp_simple_firearm 0))
                  (:NewEnumerator2
                    (Variables|/Game/WeaponMaster/Blueprints/Basic/BP_SimpleFirearm.BP_SimpleFirearm_C|SetCurrentIronsightAttachment _asbp_simple_firearm 0)))
                (Variables|DoNotTouch|SetWeaponParent 0)
                (goto _label))
              (:CastFailed
                (Development|PrintString "Not PhysMagWeap" false)))))))))

(fn ResetAttachmentZones
  (params (InteractionObject :type BP%20Interaction%20Object%20Object%20Reference))
  ;[1 1 1] Turn off attachment zones on weapons when dropped or attached.
  (switch Utilities|FlowControl|Switch|SwitchonEnum_ObjectTypes (Variables|/Game/WeaponMaster/Blueprints/Basic/BP_InteractionObject.BP_InteractionObject_C|GetObjectType InteractionObject)
    (:NewEnumerator0
      (bind _asbp_advanced_firearm (Utilities|Casting|CastToBP_AdvancedFirearm InteractionObject)
        (:then
          (Default|TurnOffAttachmentZones _asbp_advanced_firearm))
        (:CastFailed
          (Development|PrintString "Not PhysMagWeap" false))))
    (:NewEnumerator1
      (bind _asbp_simple_firearm (Utilities|Casting|CastToBP_SimpleFirearm InteractionObject)
        (:then
          (Default|TurnOffAttachmentZones _asbp_simple_firearm))
        (:CastFailed
          (Development|PrintString "Not SimpleFirearm" false))))))

(fn CheckCanRemove
  (bind _weaponparent (Variables|DoNotTouch|GetWeaponParent))
  ;[1 1 1] Check to see if the weapon allows us to remove attachments.
  (Utilities|IsValid _weaponparent
    (:Is%20Valid
      (switch Utilities|FlowControl|Switch|SwitchonEnum_ObjectTypes (Variables|/Game/WeaponMaster/Blueprints/Basic/BP_InteractionObject.BP_InteractionObject_C|GetObjectType _weaponparent)
        (:NewEnumerator0
          (bind _asbp_advanced_firearm (Utilities|Casting|CastToBP_AdvancedFirearm _weaponparent)
            (:then
              (return (Variables|/Game/WeaponMaster/Blueprints/Basic/BP_AdvancedFirearm.BP_AdvancedFirearm_C|GetbCanAddRemoveAttachments _asbp_advanced_firearm)))
            (:CastFailed
              _)))
        (:NewEnumerator1
          (bind _asbp_simple_firearm (Utilities|Casting|CastToBP_SimpleFirearm _weaponparent)
            (:then
              (return (Variables|/Game/WeaponMaster/Blueprints/Basic/BP_SimpleFirearm.BP_SimpleFirearm_C|GetbCanAddRemoveAttachments _asbp_simple_firearm)))
            (:CastFailed
              _)))
        (:NewEnumerator5
          _)
        (:NewEnumerator6
          _)
        (:NewEnumerator8
          _)
        (:NewEnumerator7
          _)))
    (:Is%20Not%20Valid
      _))
  (return false))

(fn CheckOppositeHandforWeapon
  (bind _parent (Variables|Default|GetParent))
  (bind _parent_2 (Variables|Default|GetParent))
  (bind _righthand (Variables|/Game/WeaponMaster/Blueprints/Basic/BP_VRCharacter.BP_VRCharacter_C|GetRightHand _parent_2))
  (bind _lefthand (Variables|/Game/WeaponMaster/Blueprints/Basic/BP_VRCharacter.BP_VRCharacter_C|GetLeftHand _parent))
  (bind _attachedactor (Variables|/Game/WeaponMaster/VirtualRealityBP/Blueprints/BP_MotionController.BP_MotionController_C|GetAttachedActor _lefthand))
  (bind _attachedactor_2 (Variables|/Game/WeaponMaster/VirtualRealityBP/Blueprints/BP_MotionController.BP_MotionController_C|GetAttachedActor _righthand))
  ;[1 1 1] Check to see if there is a weapon in the other hand and then show attachment zone if there is.
  (switch Utilities|FlowControl|Switch|SwitchonEControllerHand (Variables|/Game/WeaponMaster/VirtualRealityBP/Blueprints/BP_MotionController.BP_MotionController_C|GetHand (Variables|Default|GetParentHand))
    (:Left
      (Utilities|IsValid _attachedactor_2
        (:Is%20Valid
          (LocalVariables|SetLocalActor _attachedactor_2))))
    (:Right
      (Utilities|IsValid _attachedactor
        (:Is%20Valid
          (LocalVariables|SetLocalActor _attachedactor)))))
  (bind _asbp_interaction_object (Utilities|Casting|CastToBP_InteractionObject (LocalVariables|GetLocalActor))
    (:then
      (switch Utilities|FlowControl|Switch|SwitchonEnum_ObjectTypes (Variables|/Game/WeaponMaster/Blueprints/Basic/BP_InteractionObject.BP_InteractionObject_C|GetObjectType _asbp_interaction_object)
        (:NewEnumerator0
          (bind _asbp_advanced_firearm (Utilities|Casting|CastToBP_AdvancedFirearm _asbp_interaction_object))
          (Default|SetAttachmentZoneVisibility _asbp_advanced_firearm (Variables|AttachmentSetup|GetAttachmentType) true))
        (:NewEnumerator1
          (bind _asbp_simple_firearm (Utilities|Casting|CastToBP_SimpleFirearm _asbp_interaction_object))
          (Default|SetAttachmentZoneVisibility _asbp_simple_firearm (Variables|AttachmentSetup|GetAttachmentType) true))))
    (:CastFailed
      (Development|PrintString "Error:Not BP_InteractionObject" false))))