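; Ironsight weapon attachment that shows its front and extra parts only while mounted on a weapon.
; It toggles two named skeletal mesh bones, hiding them on BeginPlay without a valid parent weapon, when grabbed by a hand, and on detach.
; Attaching to a weapon unhides both bones.
; BeginPlay, Grab and attach extend the parent logic, while the detach event makes no parent call.
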(event EventBeginPlay
  ;[1 1 1] Begin Play
  (|CallParentFunction)
  (Utilities|IsValid (Variables|Default|GetWeaponParent)
    (:Is%20Not%20Valid
      (Components|SkinnedMesh|HideBonebyName (Variables|Default|GetSkeletalMesh) (Variables|AttachmentSetup|GetFrontBoneName) "PBO_None")
      (Components|SkinnedMesh|HideBonebyName (Variables|Default|GetSkeletalMesh) (Variables|AttachmentSetup|GetExtraBoneName) "PBO_None"))))

(event EventDetachedfromWeapon
  ;[1 1 1] Called when detached from a weapon
  (Components|SkinnedMesh|HideBonebyName (Variables|Default|GetSkeletalMesh) (Variables|AttachmentSetup|GetFrontBoneName) "PBO_None")
  (Components|SkinnedMesh|HideBonebyName (Variables|Default|GetSkeletalMesh) (Variables|AttachmentSetup|GetExtraBoneName) "PBO_None"))

(event EventGrab
  (params (Parent :type BP%20VR%20Character%20Object%20Reference) (Hand :type BP%20VR%20Character%20Hand%20Object%20Reference) (AttachPoint :type Scene%20Component%20Object%20Reference))
  ;[1 1 1] Grab
  (|CallParentFunction Parent Hand AttachPoint)
  (Variables|Default|SetbAttachedToHand true)
  (Components|SkinnedMesh|HideBonebyName (Variables|Default|GetSkeletalMesh) (Variables|AttachmentSetup|GetFrontBoneName) "PBO_None")
  (Components|SkinnedMesh|HideBonebyName (Variables|Default|GetSkeletalMesh) (Variables|AttachmentSetup|GetExtraBoneName) "PBO_None"))

(event EventAttachedtoWeapon
  ;[1 1 1] Called when attached to a weapon
  (|CallParentFunction)
  (Components|SkinnedMesh|UnHideBonebyName (Variables|Default|GetSkeletalMesh) (Variables|AttachmentSetup|GetFrontBoneName))
  (Components|SkinnedMesh|UnHideBonebyName (Variables|Default|GetSkeletalMesh) (Variables|AttachmentSetup|GetExtraBoneName)))

(fn ConstructionScript
  (|CallParentFunction))