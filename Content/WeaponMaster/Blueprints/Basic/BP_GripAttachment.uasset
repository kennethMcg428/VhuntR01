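; BP_GripAttachment is a grip attachment for weapons that can be grabbed by hand.
; It is a child Blueprint that forwards construction, BeginPlay, Grab and weapon attach to its parent.
; Grab also flags it as attached to a hand.
; On weapon detach it hides its OffHand component, without propagating to children or calling the parent.
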(event EventBeginPlay
  ;[1 1 1] Begin Play
  (|CallParentFunction))

(event EventDetachedfromWeapon
  ;[1 1 1] Called when detached from a weapon
  (Rendering|SetVisibility (Variables|Default|GetOffHand) false false))

(event EventGrab
  (params (Parent :type BP%20VR%20Character%20Object%20Reference) (Hand :type BP%20VR%20Character%20Hand%20Object%20Reference) (AttachPoint :type Scene%20Component%20Object%20Reference))
  ;[1 1 1] Grab
  (|CallParentFunction Parent Hand AttachPoint)
  (Variables|Default|SetbAttachedToHand true))

(event EventAttachedtoWeapon
  ;[1 1 1] Called when attached to a weapon
  (|CallParentFunction))

(fn ConstructionScript
  (|CallParentFunction))