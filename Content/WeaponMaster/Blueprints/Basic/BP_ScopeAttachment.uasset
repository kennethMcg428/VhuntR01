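; Weapon scope attachment that provides either a magnified render-target view or a plain lens, zeroed to a set distance.
; Construction snaps the scene capture and lens to mesh sockets.
; With magnification on, BeginPlay feeds the capture into a dynamic material on the scope mesh.
; When attached to an advanced firearm, ZeroScope places a sphere along the muzzle's forward line, then pitches the capture or lens toward it.
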(event EventBeginPlay
  ;[1 1 1] On begin play we need to create a render target and dynamic material before setting texture parameter and material
  (|CallParentFunction)
  (if (Variables|BasicSetup|GetbUseMagnification)
    (bind _returnvalue (Rendering|CreateRenderTarget2D 512 512))
    (bind _output_get (Variables|DoNotTouch|SetRenderTarget _returnvalue))
    (Variables|/Script/Engine.SceneCaptureComponent2D|SetTextureTarget (Variables|Default|GetSceneCaptureComponent2D) _output_get)
    (bind _returnvalue_2 (Rendering|Material|CreateDynamicMaterialInstance (Variables|MagnifierSetup|GetMasterMaterialInstance) :!class /Script/Engine.KismetMaterialLibrary))
    (Variables|DoNotTouch|SetScopeMaterial _returnvalue_2)
    (Rendering|Material|SetTextureParameterValue _returnvalue_2 (Variables|MagnifierSetup|GetTextureParameterName) (Variables|DoNotTouch|GetRenderTarget))
    (Rendering|Material|SetMaterialbyName (Variables|Default|GetSkeletalMesh) (Variables|MagnifierSetup|GetSlotName) (Variables|DoNotTouch|GetScopeMaterial))))

(event EventAttachedtoWeapon
  (CallFunction|ZeroScope))

(fn ConstructionScript
  (bind _lens (Variables|Default|GetLens))
  ;[1 1 1] Attach scene capture component to correct socket
  (|CallParentFunction)
  (Transformation|AttachComponentToComponent (Variables|Default|GetSceneCaptureComponent2D) (Variables|Default|GetSkeletalMesh) (Variables|MagnifierSetup|GetCameraSocket) "SnapToTarget" "SnapToTarget" "KeepWorld" true)
  (Utilities|IsValid _lens
    (:Is%20Valid
      (Transformation|AttachComponentToComponent _lens (Variables|Default|GetSkeletalMesh) (Variables|1xSetup|GetLensSocket) "SnapToTarget" "SnapToTarget" "KeepWorld" true))))

(fn ZeroScope
  (bind _scenecapturecomponent2d (Variables|Default|GetSceneCaptureComponent2D))
  (bind _lens (Variables|Default|GetLens))
  (bind _returnvalue (Transformation|GetWorldRotation _lens))
  (bind _returnvalue_2 (Transformation|GetWorldRotation _scenecapturecomponent2d))
  (bind (_roll _pitch _yaw) (Math|Rotator|BreakRotator _returnvalue_2))
  (bind (_roll_2 _pitch_2 _yaw_2) (Math|Rotator|BreakRotator _returnvalue))
  (bind _asbp_advanced_firearm (Utilities|Casting|CastToBP_AdvancedFirearm (Variables|Default|GetWeaponParent)))
  (switch Utilities|FlowControl|Switch|SwitchonEnum_ZeroUnits (Variables|BasicSetup|GetZeroUnits)
    (:NewEnumerator0
      (LocalVariables|SetActualDistance (* (Variables|BasicSetup|GetZeroDistance) 91.44)))
    (:NewEnumerator1
      (LocalVariables|SetActualDistance (* (Variables|BasicSetup|GetZeroDistance) 1e+02))))
  (Transformation|SetWorldLocation (Variables|Default|GetSphere) (+ (Transformation|GetSocketLocation (Variables|/Game/WeaponMaster/Blueprints/Basic/BP_BasicFirearmPickup.BP_BasicFirearmPickup_C|GetSkeletalMesh _asbp_advanced_firearm) (Variables|/Game/WeaponMaster/Blueprints/Basic/BP_AdvancedFirearm.BP_AdvancedFirearm_C|GetMuzzleSocket _asbp_advanced_firearm)) (* (Math|Vector|GetForwardVector (Transformation|GetSocketRotation (Variables|/Game/WeaponMaster/Blueprints/Basic/BP_BasicFirearmPickup.BP_BasicFirearmPickup_C|GetSkeletalMesh _asbp_advanced_firearm) (Variables|/Game/WeaponMaster/Blueprints/Basic/BP_AdvancedFirearm.BP_AdvancedFirearm_C|GetMuzzleSocket _asbp_advanced_firearm))) (LocalVariables|GetActualDistance))) false false)
  (if (Variables|BasicSetup|GetbUseMagnification)
    (Transformation|SetWorldRotation _scenecapturecomponent2d (Math|Rotator|MakeRotator _roll (.Pitch (Math|Rotator|BreakRotator (Math|Rotator|FindLookatRotation (Transformation|GetWorldLocation _scenecapturecomponent2d) (Transformation|GetWorldLocation (Variables|Default|GetSphere))))) _yaw) false false)
    (else
      (Transformation|SetWorldRotation _lens (Math|Rotator|MakeRotator _roll_2 (.Pitch (Math|Rotator|BreakRotator (Math|Rotator|FindLookatRotation (Transformation|GetWorldLocation _lens) (Transformation|GetWorldLocation (Variables|Default|GetSphere))))) _yaw_2) false false))))