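; BP_Effect is a basic effect actor that spawns particle effects where it is placed or spawned.
; On Begin Play it spawns the Particle emitter at the actor's location and rotation, then a second one from Particle2 if Use2ndParticle is set.
; Each template is validity-checked, and the emitters are spawned at the location rather than attached, with no cleanup logic in the actor.
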(event EventBeginPlay
  (bind _returnvalue (Transformation|GetActorTransform))
  (bind _returnvalue_2 (Transformation|GetActorTransform))
  (bind _particle (Variables|Default|GetParticle))
  (bind _particle2 (Variables|Default|GetParticle2))
  (bind (_location _rotation) (Math|Transform|BreakTransform _returnvalue))
  (bind (_location_2 _rotation_2) (Math|Transform|BreakTransform _returnvalue_2))
  ;[1 1 1] Begin Play
  ;;[1 1 1] Spawn first Particle at actor location
  (Utilities|IsValid _particle
    (:Is%20Valid
      (Effects|SpawnEmitteratLocation _particle _location_2 _rotation_2))
    (:Is%20Not%20Valid
      _))
  ;;[1 1 1] Spawn second particle if desired.
  (if (Variables|Default|GetbUse2ndParticle)
    (Utilities|IsValid _particle2
      (:Is%20Valid
        (Effects|SpawnEmitteratLocation _particle2 _location _rotation)))))

(fn ConstructionScript)