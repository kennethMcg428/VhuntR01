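; Survival game mode that runs ten zombie waves of rising count and difficulty, then plays a win cue.
; NextWave sets each wave's caps, resets counters, plays its cue and assigns the zombie type to every attack spawner.
; Spawn and kill events update counters that CheckCanSpawn tests; kills also call DoScore and trigger wave advancement.
; When one counted zombie remains, a world search advances the wave if no melee AI exists, covering miscounts.
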(event Custom|ZombieKilled
  (params (bHeadshot :type Boolean))
  ;[1 1 1] If a zombie is killed subtract 1 from the level amount and then check if the round is over before incrementing score.
  (Variables|Default|SetCurrentZombiesInLevel (- (Variables|Default|GetCurrentZombiesInLevel) 1))
  (if (and (>= (Variables|Default|GetCurrentZombiesSpawned) (Variables|Default|GetMaxZombiesForWave)) (<= (Variables|Default|GetCurrentZombiesInLevel) 0))
    (CallFunction|NextWave)
    (elif (== (Variables|Default|GetCurrentZombiesInLevel) 1)
      (CallFunction|CheckMapforLastZombie)))
  (CallFunction|DoScore bHeadshot))

(event Custom|CheckMapForLastZombie
  ;[1 1 1] Check and make sure we didnt miss a zombie
  (bind _outactors (Actor|GetAllActorsOfClass "/Game/WeaponMaster/AI/BP_MeleeAI_Character.BP_MeleeAI_Character_C"))
  (if (not (Utilities|Array|IsValidIndex _outactors))
    (CallFunction|NextWave)))

(event Custom|ZombieSpawned
  (params (ZombieSpawned :type BP%20Melee%20AI%20Character%20Object%20Reference))
  ;[1 1 1] Increment values when zombie is spawned
  (Utilities|IsValid ZombieSpawned
    (:Is%20Valid
      (Variables|Default|SetCurrentZombiesInLevel (+ (Variables|Default|GetCurrentZombiesInLevel) 1))
      (Variables|Default|SetCurrentZombiesSpawned (+ (Variables|Default|GetCurrentZombiesSpawned) 1)))))

(event EventBeginPlay
  ;[1 1 1] Start on wave 1 (int 1)
  (CallFunction|NextWave))

(fn ConstructionScript
  (|CallParentFunction))

(fn CheckCanSpawn
  ;[1 1 1] Check to see if we can spawn another zombie
  (if (and (< (Variables|Default|GetCurrentZombiesSpawned) (Variables|Default|GetMaxZombiesForWave)) (< (Variables|Default|GetCurrentZombiesInLevel) (Variables|Default|GetMaxZombiesInLevel)))
    (return true)
    (else
      (return false))))

(fn NextWave
  ;[1 1 1] Iterate through waves setting the correct MaxZombiesForWave and MaxZombiesInLevel for each
  (Variables|Default|SetWave (+ (Variables|Default|GetWave) 1))
  (switch int (Variables|Default|GetWave)
    (:1
      (CallFunction|UpdateSpawners (Variables|Default|GetEasyZombie))
      (Audio|PlaySound2D "/Game/WeaponMaster/Audio/Announcer/Cue_Wave1.Cue_Wave1")
      (Variables|Default|SetMaxZombiesForWave 10)
      (Variables|Default|SetMaxZombiesInLevel 5)
      (Variables|Default|SetCurrentZombiesInLevel 0 :!label _label)
      (Variables|Default|SetCurrentZombiesSpawned 0))
    (:2
      (CallFunction|UpdateSpawners (Variables|Default|GetEasyZombie))
      (Audio|PlaySound2D "/Game/WeaponMaster/Audio/Announcer/Cue_Wave2.Cue_Wave2")
      (Variables|Default|SetMaxZombiesForWave 15)
      (Variables|Default|SetMaxZombiesInLevel 10)
      (goto _label))
    (:3
      (CallFunction|UpdateSpawners (Variables|Default|GetMediumZombie))
      (Audio|PlaySound2D "/Game/WeaponMaster/Audio/Announcer/Cue_Wave3.Cue_Wave3")
      (Variables|Default|SetMaxZombiesForWave 20)
      (Variables|Default|SetMaxZombiesInLevel 10)
      (goto _label))
    (:4
      (CallFunction|UpdateSpawners (Variables|Default|GetMediumZombie))
      (Audio|PlaySound2D "/Game/WeaponMaster/Audio/Announcer/Cue_Wave4.Cue_Wave4")
      (Variables|Default|SetMaxZombiesForWave 25)
      (Variables|Default|SetMaxZombiesInLevel 10)
      (goto _label))
    (:5
      (CallFunction|UpdateSpawners (Variables|Default|GetMediumZombie))
      (Audio|PlaySound2D "/Game/WeaponMaster/Audio/Announcer/Cue_Wave5.Cue_Wave5")
      (Variables|Default|SetMaxZombiesForWave 30)
      (Variables|Default|SetMaxZombiesInLevel 15)
      (goto _label))
    (:6
      (CallFunction|UpdateSpawners (Variables|Default|GetMediumZombie))
      (Audio|PlaySound2D "/Game/WeaponMaster/Audio/Announcer/Cue_Wave6.Cue_Wave6")
      (Variables|Default|SetMaxZombiesForWave 35)
      (Variables|Default|SetMaxZombiesInLevel 15)
      (goto _label))
    (:7
      (CallFunction|UpdateSpawners (Variables|Default|GetHardZombie))
      (Audio|PlaySound2D "/Game/WeaponMaster/Audio/Announcer/Cue_Wave7.Cue_Wave7")
      (Variables|Default|SetMaxZombiesForWave 40)
      (Variables|Default|SetMaxZombiesInLevel 20)
      (goto _label))
    (:8
      (CallFunction|UpdateSpawners (Variables|Default|GetHardZombie))
      (Audio|PlaySound2D "/Game/WeaponMaster/Audio/Announcer/Cue_Wave8.Cue_Wave8")
      (Variables|Default|SetMaxZombiesForWave 45)
      (Variables|Default|SetMaxZombiesInLevel 20)
      (goto _label))
    (:9
      (CallFunction|UpdateSpawners (Variables|Default|GetHardZombie))
      (Audio|PlaySound2D "/Game/WeaponMaster/Audio/Announcer/Cue_Wave9.Cue_Wave9")
      (Variables|Default|SetMaxZombiesForWave 50)
      (Variables|Default|SetMaxZombiesInLevel 20)
      (goto _label))
    (:10
      (CallFunction|UpdateSpawners (Variables|Default|GetHardZombie))
      (Audio|PlaySound2D "/Game/WeaponMaster/Audio/Announcer/Cue_FinalWave.Cue_FinalWave")
      (Variables|Default|SetMaxZombiesForWave 60)
      (Variables|Default|SetMaxZombiesInLevel 20)
      (goto _label))
    (:11
      (Audio|PlaySound2D "/Game/WeaponMaster/Audio/Announcer/Cue_Win.Cue_Win"))))

(fn UpdateSpawners
  (params (WaveZombie :type BP%20Melee%20AI%20Character%20Class%20Reference))
  ;[1 1 1] Find all spawners and change what zombies they are supposed to spawn
  (bind _outactors (Actor|GetAllActorsOfClass "/Game/WeaponMaster/AI/BP_AI_ZombieAttackSpawner.BP_AI_ZombieAttackSpawner_C"))
  (for _array_element _outactors
    (Variables|/Game/WeaponMaster/AI/BP_AI_Spawner.BP_AI_Spawner_C|SetAIToSpawn _array_element WaveZombie)))