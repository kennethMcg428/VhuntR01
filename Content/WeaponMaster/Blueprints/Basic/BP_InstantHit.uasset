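; Instant-hit weapon shot actor that runs one complex line trace on BeginPlay and resolves the impact.
; The hit's physical surface type selects a random decal class, particle effect and sound from per-surface arrays.
; Decal actors spawn only on WorldStatic or one custom object channel.
; Point damage follows, with LocalDamage computed only for Flesh and Head surfaces, the latter scaled by a critical multiplier.
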(event EventBeginPlay
  (bind _defaultimpactsounds (Variables|Default|GetDefaultImpactSounds))
  (bind _woodimpactsounds (Variables|Default|GetWoodImpactSounds))
  (bind _concreteimpactsounds (Variables|Default|GetConcreteImpactSounds))
  (bind _plasterimpactsounds (Variables|Default|GetPlasterImpactSounds))
  (bind _metalimpactsounds (Variables|Default|GetMetalImpactSounds))
  (bind _grassimpactsounds (Variables|Default|GetGrassImpactSounds))
  (bind _fleshimpactsounds (Variables|Default|GetFleshImpactSounds))
  (bind _fleshimpactsounds_2 (Variables|Default|GetFleshImpactSounds))
  (bind _defaulteffects (Variables|Default|GetDefaultEffects))
  (bind _defaultdecals (Variables|Default|GetDefaultDecals))
  (bind _flesheffects (Variables|Default|GetFleshEffects))
  (bind _wooddecals (Variables|Default|GetWoodDecals))
  (bind _woodeffects (Variables|Default|GetWoodEffects))
  (bind _concretedecals (Variables|Default|GetConcreteDecals))
  (bind _concreteeffects (Variables|Default|GetConcreteEffects))
  (bind _plasterdecals (Variables|Default|GetPlasterDecals))
  (bind _plastereffects (Variables|Default|GetPlasterEffects))
  (bind _metaldecals (Variables|Default|GetMetalDecals))
  (bind _metaleffects (Variables|Default|GetMetalEffects))
  (bind _grasseffects (Variables|Default|GetGrassEffects))
  (bind _grassdecals (Variables|Default|GetGrassDecals))
  (bind _flesheffects_2 (Variables|Default|GetFleshEffects))
  (bind _tiledecals (Variables|Default|GetTileDecals))
  (bind _tileeffects (Variables|Default|GetTileEffects))
  (bind _tileimpactsounds (Variables|Default|GetTileImpactSounds))
  (bind _clothdecals (Variables|Default|GetClothDecals))
  (bind _clotheffects (Variables|Default|GetClothEffects))
  (bind _clothimpactsounds (Variables|Default|GetClothImpactSounds))
  (bind _dirtdecals (Variables|Default|GetDirtDecals))
  (bind _dirteffects (Variables|Default|GetDirtEffects))
  (bind _dirtimpactsounds (Variables|Default|GetDirtImpactSounds))
  ;[1 1 1] Linetrace to find hit, set variables and deside physic mat hit.
  (bind _outhit (Collision|LineTraceByChannel (Variables|Default|GetStartLocation) (Variables|Default|GetEndLocation) "TraceTypeQuery3" true (Utilities|Array|MakeArray (Variables|Default|GetInstigator) (Components|GetOwner)) "None"))
  (if (.bBlockingHit (Collision|BreakHitResult _outhit))
    (Variables|DoNotTouch|SetLocalHit _outhit)
    (Variables|DoNotTouch|SetLocalLocation (.Location (Collision|BreakHitResult _outhit)))
    (Variables|DoNotTouch|SetLocalNormal (.ImpactNormal (Collision|BreakHitResult _outhit)))
    (Variables|DoNotTouch|SetLocalComponent (.HitComponent (Collision|BreakHitResult _outhit)))
    (Variables|DoNotTouch|SetHitActor (.HitActor (Collision|BreakHitResult _outhit)))
    (Variables|DoNotTouch|SetHitDirection (Math|Vector|GetUnitDirection(Vector) (.TraceStart (Collision|BreakHitResult _outhit)) (.Location (Collision|BreakHitResult _outhit))))
    (switch Utilities|FlowControl|Switch|SwitchonEPhysicalSurface (Variables|/Script/Engine.PhysicalMaterial|GetSurfaceType (.PhysMat (Collision|BreakHitResult _outhit)))
      (:SurfaceType_Default
        ;[1 1 1] Deside Damage then, from their specific arrays pic 1 decal, effect and sound to spawn.
        (if (> (Utilities|Array|Length (Variables|Default|GetDefaultDecals)) 0)
          (Variables|DoNotTouch|SetDecalMaterial (Utilities|Array|Get(acopy) _defaultdecals (Math|Random|RandomInteger (Utilities|Array|Length _defaultdecals)))))
        (if (> (Utilities|Array|Length (Variables|Default|GetDefaultEffects)) 0)
          (Variables|DoNotTouch|SetImpactEffect (Utilities|Array|Get(acopy) _defaulteffects (Math|Random|RandomInteger (Utilities|Array|Length _defaulteffects)))))
        (if (> (Utilities|Array|Length (Variables|Default|GetDefaultImpactSounds)) 0)
          (Variables|DoNotTouch|SetImpactSound (Utilities|Array|Get(acopy) _defaultimpactsounds (Math|Random|RandomInteger (Utilities|Array|Length _defaultimpactsounds))))))
      (:SurfaceType1
        (Variables|DoNotTouch|SetLocalDamage (+ (Variables|Default|GetDamage) (Variables|Default|GetWeaponDamageModifier)))
        (if (> (Utilities|Array|Length (Variables|Default|GetFleshEffects)) 0)
          (Variables|DoNotTouch|SetImpactEffect (Utilities|Array|Get(acopy) _flesheffects_2 (Math|Random|RandomInteger (Utilities|Array|Length _flesheffects_2)))))
        (if (> (Utilities|Array|Length (Variables|Default|GetFleshImpactSounds)) 0)
          (Variables|DoNotTouch|SetImpactSound (Utilities|Array|Get(acopy) _fleshimpactsounds (Math|Random|RandomInteger (Utilities|Array|Length _fleshimpactsounds))))))
      (:SurfaceType2
        (if (> (Utilities|Array|Length (Variables|Default|GetWoodDecals)) 0)
          (Variables|DoNotTouch|SetDecalMaterial (Utilities|Array|Get(acopy) _wooddecals (Math|Random|RandomInteger (Utilities|Array|Length _wooddecals)))))
        (if (> (Utilities|Array|Length (Variables|Default|GetWoodEffects)) 0)
          (Variables|DoNotTouch|SetImpactEffect (Utilities|Array|Get(acopy) _woodeffects (Math|Random|RandomInteger (Utilities|Array|Length _woodeffects)))))
        (if (>= (Utilities|Array|Length (Variables|Default|GetWoodImpactSounds)) 0)
          (Variables|DoNotTouch|SetImpactSound (Utilities|Array|Get(acopy) _woodimpactsounds (Math|Random|RandomInteger (Utilities|Array|Length _woodimpactsounds))))))
      (:SurfaceType3
        (if (> (Utilities|Array|Length (Variables|Default|GetConcreteDecals)) 0)
          (Variables|DoNotTouch|SetDecalMaterial (Utilities|Array|Get(acopy) _concretedecals (Math|Random|RandomInteger (Utilities|Array|Length _concretedecals)))))
        (if (> (Utilities|Array|Length (Variables|Default|GetConcreteEffects)) 0)
          (Variables|DoNotTouch|SetImpactEffect (Utilities|Array|Get(acopy) _concreteeffects (Math|Random|RandomInteger (Utilities|Array|Length _concreteeffects)))))
        (if (> (Utilities|Array|Length (Variables|Default|GetConcreteImpactSounds)) 0)
          (Variables|DoNotTouch|SetImpactSound (Utilities|Array|Get(acopy) _concreteimpactsounds (Math|Random|RandomInteger (Utilities|Array|Length _concreteimpactsounds))))))
      (:SurfaceType4
        (if (> (Utilities|Array|Length (Variables|Default|GetPlasterDecals)) 0)
          (Variables|DoNotTouch|SetDecalMaterial (Utilities|Array|Get(acopy) _plasterdecals (Math|Random|RandomInteger (Utilities|Array|Length _plasterdecals)))))
        (if (> (Utilities|Array|Length (Variables|Default|GetPlasterEffects)) 0)
          (Variables|DoNotTouch|SetImpactEffect (Utilities|Array|Get(acopy) _plastereffects (Math|Random|RandomInteger (Utilities|Array|Length _plastereffects)))))
        (if (> (Utilities|Array|Length (Variables|Default|GetPlasterImpactSounds)) 0)
          (Variables|DoNotTouch|SetImpactSound (Utilities|Array|Get(acopy) _plasterimpactsounds (Math|Random|RandomInteger (Utilities|Array|Length _plasterimpactsounds))))))
      (:SurfaceType5
        (if (> (Utilities|Array|Length (Variables|Default|GetMetalDecals)) 0)
          (Variables|DoNotTouch|SetDecalMaterial (Utilities|Array|Get(acopy) _metaldecals (Math|Random|RandomInteger (Utilities|Array|Length _metaldecals)))))
        (if (> (Utilities|Array|Length (Variables|Default|GetMetalEffects)) 0)
          (Variables|DoNotTouch|SetImpactEffect (Utilities|Array|Get(acopy) _metaleffects (Math|Random|RandomInteger (Utilities|Array|Length _metaleffects)))))
        (if (> (Utilities|Array|Length (Variables|Default|GetMetalImpactSounds)) 0)
          (Variables|DoNotTouch|SetImpactSound (Utilities|Array|Get(acopy) _metalimpactsounds (Math|Random|RandomInteger (Utilities|Array|Length _metalimpactsounds))))))
      (:SurfaceType6
        (if (> (Utilities|Array|Length (Variables|Default|GetGrassDecals)) 0)
          (Variables|DoNotTouch|SetDecalMaterial (Utilities|Array|Get(acopy) _grassdecals (Math|Random|RandomInteger (Utilities|Array|Length _grassdecals)))))
        (if (> (Utilities|Array|Length (Variables|Default|GetGrassEffects)) 0)
          (Variables|DoNotTouch|SetImpactEffect (Utilities|Array|Get(acopy) _grasseffects (Math|Random|RandomInteger (Utilities|Array|Length _grasseffects)))))
        (if (> (Utilities|Array|Length (Variables|Default|GetGrassImpactSounds)) 0)
          (Variables|DoNotTouch|SetImpactSound (Utilities|Array|Get(acopy) _grassimpactsounds (Math|Random|RandomInteger (Utilities|Array|Length _grassimpactsounds))))))
      (:SurfaceType7
        (Variables|DoNotTouch|SetLocalDamage (* (+ (Variables|Default|GetDamage) (Variables|Default|GetWeaponDamageModifier)) (Variables|Default|GetCriticalMultiplier)))
        (if (> (Utilities|Array|Length (Variables|Default|GetFleshEffects)) 0)
          (Variables|DoNotTouch|SetImpactEffect (Utilities|Array|Get(acopy) _flesheffects (Math|Random|RandomInteger (Utilities|Array|Length _flesheffects)))))
        (if (> (Utilities|Array|Length (Variables|Default|GetFleshImpactSounds)) 0)
          (Variables|DoNotTouch|SetImpactSound (Utilities|Array|Get(acopy) _fleshimpactsounds_2 (Math|Random|RandomInteger (Utilities|Array|Length _fleshimpactsounds_2))))))
      (:SurfaceType8
        (if (> (Utilities|Array|Length (Variables|Default|GetTileDecals)) 0)
          (Variables|DoNotTouch|SetDecalMaterial (Utilities|Array|Get(acopy) _tiledecals (Math|Random|RandomInteger (Utilities|Array|Length _tiledecals)))))
        (if (> (Utilities|Array|Length (Variables|Default|GetTileEffects)) 0)
          (Variables|DoNotTouch|SetImpactEffect (Utilities|Array|Get(acopy) _tileeffects (Math|Random|RandomInteger (Utilities|Array|Length _tileeffects)))))
        (if (> (Utilities|Array|Length (Variables|Default|GetTileImpactSounds)) 0)
          (Variables|DoNotTouch|SetImpactSound (Utilities|Array|Get(acopy) _tileimpactsounds (Math|Random|RandomInteger (Utilities|Array|Length _tileimpactsounds))))))
      (:SurfaceType9
        (if (> (Utilities|Array|Length (Variables|Default|GetClothDecals)) 0)
          (Variables|DoNotTouch|SetDecalMaterial (Utilities|Array|Get(acopy) _clothdecals (Math|Random|RandomInteger (Utilities|Array|Length _clothdecals)))))
        (if (> (Utilities|Array|Length (Variables|Default|GetClothEffects)) 0)
          (Variables|DoNotTouch|SetImpactEffect (Utilities|Array|Get(acopy) _clotheffects (Math|Random|RandomInteger (Utilities|Array|Length _clotheffects)))))
        (if (> (Utilities|Array|Length (Variables|Default|GetClothImpactSounds)) 0)
          (Variables|DoNotTouch|SetImpactSound (Utilities|Array|Get(acopy) _clothimpactsounds (Math|Random|RandomInteger (Utilities|Array|Length _clothimpactsounds))))))
      (:SurfaceType10
        (if (> (Utilities|Array|Length (Variables|Default|GetDirtDecals)) 0)
          (Variables|DoNotTouch|SetDecalMaterial (Utilities|Array|Get(acopy) _dirtdecals (Math|Random|RandomInteger (Utilities|Array|Length _dirtdecals)))))
        (if (> (Utilities|Array|Length (Variables|Default|GetDirtEffects)) 0)
          (Variables|DoNotTouch|SetImpactEffect (Utilities|Array|Get(acopy) _dirteffects (Math|Random|RandomInteger (Utilities|Array|Length _dirteffects)))))
        (if (> (Utilities|Array|Length (Variables|Default|GetDirtImpactSounds)) 0)
          (Variables|DoNotTouch|SetImpactSound (Utilities|Array|Get(acopy) _dirtimpactsounds (Math|Random|RandomInteger (Utilities|Array|Length _dirtimpactsounds)))))))
    ;[1 1 1] Spawn selected Decal, Impact Effect and Impact Sound
    (if (Utilities|IsValidClass (Variables|DoNotTouch|GetDecalMaterial))
      (if (or (Utilities|Enum|Equal(Enum) (Collision|GetCollisionObjectType (Variables|DoNotTouch|GetLocalComponent)) "ECC_WorldStatic") (Utilities|Enum|Equal(Enum) (Collision|GetCollisionObjectType (Variables|DoNotTouch|GetLocalComponent)) "ECC_GameTraceChannel17"))
        (bind _returnvalue (Game|SpawnActorfromClass (Variables|DoNotTouch|GetDecalMaterial) (Math|Transform|MakeTransform (Variables|DoNotTouch|GetLocalLocation) (Math|Rotator|MakeRotfromX (Variables|DoNotTouch|GetLocalNormal))) "AlwaysSpawn" 0 0))
        (Transformation|SetActorRotation _returnvalue (Math|Rotator|MakeRotfromX (Variables|DoNotTouch|GetLocalNormal)))))
    (Utilities|IsValid (Variables|DoNotTouch|GetImpactSound)
      (:Is%20Valid
        (Audio|PlaySoundatLocation (Variables|DoNotTouch|GetImpactSound) (Variables|DoNotTouch|GetLocalLocation)))
      (:Is%20Not%20Valid
        _))
    (Utilities|IsValid (Variables|DoNotTouch|GetImpactEffect)
      (:Is%20Valid
        (Effects|SpawnEmitteratLocation (Variables|DoNotTouch|GetImpactEffect) (Variables|DoNotTouch|GetLocalLocation) (Math|Rotator|MakeRotfromX (Variables|DoNotTouch|GetLocalNormal))))
      (:Is%20Not%20Valid
        _))
    ;[1 1 1] Apply Damage
    (Game|Damage|ApplyPointDamage (Variables|DoNotTouch|GetHitActor) (Variables|DoNotTouch|GetLocalDamage) (Variables|DoNotTouch|GetHitDirection) (Variables|DoNotTouch|GetLocalHit) (Game|GetInstigatorController) (Components|GetOwner) (Variables|Default|GetDamageType))))

(fn ConstructionScript
  (|CallParentFunction))