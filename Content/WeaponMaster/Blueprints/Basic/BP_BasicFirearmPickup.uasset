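; Base VR firearm pickup that can be grabbed by a hand, holstered, unholstered and released.
; Grab and holster snap the root to an attach point and the mesh to a Recoil component, disabling physics and applying per-state offsets.
; Hand attachment updates the mag counter and optionally hides the hand mesh; release restores both visibility and physics.
; Holstering disables mesh overlap events to block grabbing until unholstered.
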(event EventGrab
  (params (Parent :type BP%20VR%20Character%20Object%20Reference) (Hand :type BP%20VR%20Character%20Hand%20Object%20Reference) (AttachPoint :type Scene%20Component%20Object%20Reference))
  ;[1 1 1] Hand Grab Logic
  (CallFunction|AttachtoHand Parent Hand AttachPoint))

(event EventHolster
  (params (HolsterComponent :type Skeletal%20Mesh%20Component%20Object%20Reference) (AttachPoint :type Scene%20Component%20Object%20Reference))
  ;[1 1 1] Holster Logic
  (CallFunction|AttachtoHolster HolsterComponent AttachPoint))

(event EventUnHolster
  (params (Parent :type BP%20VR%20Character%20Object%20Reference) (Hand :type BP%20VR%20Character%20Hand%20Object%20Reference) (AttachPoint :type Scene%20Component%20Object%20Reference))
  ;[1 1 1] Unholster Logic
  ;;[0 0 0] Detach from Holster first
  (CallFunction|DetachfromHolster)
  (CallFunction|AttachtoHand Parent Hand AttachPoint))

(event EventReleaseObject
  ;[1 1 1] Hand Release Logic
  (CallFunction|DetachfromHand))

(fn ConstructionScript)

(fn AttachtoHand
  (params (Parent :type BP%20VR%20Character%20Object%20Reference) (Hand :type BP%20VR%20Character%20Hand%20Object%20Reference) (AttachPoint :type Scene%20Component%20Object%20Reference))
  ;[1 1 1] Attach To Hand
  (Utilities|IsValid Parent
    (:Is%20Valid
      (Utilities|IsValid Hand
        (:Is%20Valid
          ;;[0 0 0] SetParentandHandParent
          (Variables|Default|SetParent Parent)
          (Variables|Default|SetParentHand Hand)
          (bind _output_get (Variables|Default|SetAttachPoint AttachPoint))
          ;;[0 0 0] Attach and Turn off Physics
          (Transformation|AttachComponentToComponent (Variables|Default|GetRoot) _output_get "None" "SnapToTarget" "SnapToTarget" "KeepWorld" false)
          (Physics|SetSimulatePhysics (Variables|Default|GetSkeletalMesh) false)
          (Transformation|AttachComponentToComponent (Variables|Default|GetSkeletalMesh) (Variables|Default|GetRecoil) "None" "SnapToTarget" "SnapToTarget" "KeepWorld" false)
          ;;[0 0 0] Set hand attached actor
          (Variables|/Game/WeaponMaster/VirtualRealityBP/Blueprints/BP_MotionController.BP_MotionController_C|SetAttachedActor (Variables|Default|GetParentHand) self)
          ;;[0 0 0] Clear unholster variables
          (switch Utilities|FlowControl|Switch|SwitchonEControllerHand (Variables|/Game/WeaponMaster/VirtualRealityBP/Blueprints/BP_MotionController.BP_MotionController_C|GetHand (Variables|Default|GetParentHand))
            (:Left
              (Variables|/Game/WeaponMaster/Blueprints/Basic/BP_VRCharacter.BP_VRCharacter_C|SetTempLeftUnholsterObject (Variables|Default|GetParent) 0))
            (:Right
              (Variables|/Game/WeaponMaster/Blueprints/Basic/BP_VRCharacter.BP_VRCharacter_C|SetTempRightUnholsterObject (Variables|Default|GetParent) 0)))
          ;;[0 0 0] Do location and rotation adjustments
          (Transformation|SetRelativeLocationAndRotation (Variables|Default|GetSkeletalMesh) (Variables|Default|GetHeldLocationAdjustment) (Variables|Default|GetHeldRotationAdjustment) false false)
          ;;[0 0 0] Update UI, clear HeldinOffHand, and hide Hand Parent Mesh if desired.
          (Default|UpdateMagCounter (Variables|Default|GetParent))
          (Variables|Default|SetbHeldInOffHand false)
          (if (Variables|Default|GetbHideInGameHand)
            (Rendering|SetVisibility (Variables|/Game/WeaponMaster/VirtualRealityBP/Blueprints/BP_MotionController.BP_MotionController_C|GetHandMesh (Variables|Default|GetParentHand)) false false)))))))

(fn DetachfromHand
  (bind _skeletalmesh (Variables|Default|GetSkeletalMesh))
  ;[1 1 1] Detach from hand.
  (Utilities|IsValid (Variables|Default|GetParentHand)
    (:Is%20Valid
      ;;[0 0 0] Clear Attached Actor
      (Variables|/Game/WeaponMaster/VirtualRealityBP/Blueprints/BP_MotionController.BP_MotionController_C|SetAttachedActor (Variables|Default|GetParentHand) 0)
      ;;[0 0 0] Update UI and Show Parent Hand Mesh
      (Default|UpdateMagCounter (Variables|Default|GetParent))
      (Rendering|SetVisibility (Variables|/Game/WeaponMaster/VirtualRealityBP/Blueprints/BP_MotionController.BP_MotionController_C|GetHandMesh (Variables|Default|GetParentHand)) true false)
      ;;[0 0 0] Clear variables
      (Variables|Default|SetParent 0)
      (Variables|Default|SetParentHand 0)
      (Variables|Default|SetAttachPoint 0)
      ;;[0 0 0] Detach from Hand, turn on collision and turn on simulate physics
      (Transformation|DetachFromComponent (Variables|Default|GetRoot) "KeepWorld" "KeepWorld" "KeepWorld" true)
      (Collision|SetCollisionEnabled _skeletalmesh "QueryAndPhysics")
      (Physics|SetSimulatePhysics _skeletalmesh true))))

(fn AttachtoHolster
  (params (HolsterComponent :type Skeletal%20Mesh%20Component%20Object%20Reference) (AttachPoint :type Scene%20Component%20Object%20Reference))
  ;[1 1 1] Attach to Holster
  (Utilities|IsValid HolsterComponent
    (:Is%20Valid
      (Utilities|IsValid AttachPoint
        (:Is%20Valid
          ;;[0 0 0] SetHolsterParent
          (Variables|Default|SetHolsterParent HolsterComponent)
          (bind _output_get (Variables|Default|SetAttachPoint AttachPoint))
          ;;[0 0 0] Turn off Physics
          (Physics|SetSimulatePhysics (Variables|Default|GetSkeletalMesh) false)
          ;;[0 0 0] Turn off overlap events so we cannot grab.
          (Variables|/Script/Engine.PrimitiveComponent|SetbGenerateOverlapEvents (Variables|Default|GetSkeletalMesh) false)
          ;;[0 0 0] Attach to Holster and set location and rotation adjustments
          (Transformation|AttachComponentToComponent (Variables|Default|GetRoot) _output_get "None" "SnapToTarget" "SnapToTarget" "KeepWorld" false)
          (Transformation|AttachComponentToComponent (Variables|Default|GetSkeletalMesh) (Variables|Default|GetRecoil) "None" "SnapToTarget" "SnapToTarget" "KeepWorld" false)
          (Transformation|SetRelativeLocationAndRotation (Variables|Default|GetSkeletalMesh) (Variables|Default|GetHolsterLocationAdjustment) (Variables|Default|GetHolsterRotationAdjustment) false false)
          ;;[0 0 0] Clear Varaible
          (Variables|Default|SetParentHand 0))))))

(fn DetachfromHolster
  ;[1 1 1] Detach from holster and clear variables
  (Transformation|DetachFromComponent (Variables|Default|GetRoot) "KeepWorld" "KeepWorld" "KeepWorld" false)
  ;;[0 0 0] Turn on overlap events so we can grab again
  (Variables|/Script/Engine.PrimitiveComponent|SetbGenerateOverlapEvents (Variables|Default|GetSkeletalMesh) true)
  (Variables|Default|SetHolsterParent 0)
  (Variables|Default|SetAttachPoint 0))