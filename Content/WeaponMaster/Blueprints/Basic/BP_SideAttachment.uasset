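; BP_SideAttachment is a weapon side attachment, such as a flashlight or laser, with a toggleable light.
; The construction script snaps its SpotLight to a light socket on the skeletal mesh.
; In flashlight mode, ToggleLight flips the spotlight's visibility, and detaching from the weapon hides it to save performance.
; The laser branches are empty, so only the flashlight has behavior here.
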(event Custom|ToggleLight
  ;[1 1 1] Toggle flashlight or laser visibility
  (if (Variables|AttachmentSetup|GetbIsFlashlight)
    (Rendering|ToggleVisibility (Variables|Default|GetSpotLight) false)
    (elif (Variables|AttachmentSetup|GetbIsLaser)
      _)))

(event EventDetachedfromWeapon
  ;[1 1 1] Turn off light when it is removed to help performance
  (if (Variables|AttachmentSetup|GetbIsFlashlight)
    (Rendering|SetVisibility (Variables|Default|GetSpotLight) false false)
    (elif (Variables|AttachmentSetup|GetbIsLaser)
      _)))

(fn ConstructionScript
  (|CallParentFunction)
  (Transformation|AttachComponentToComponent (Variables|Default|GetSpotLight) (Variables|Default|GetSkeletalMesh) (Variables|AttachmentSetup|GetLightSocket) "SnapToTarget" "SnapToTarget" "KeepWorld" true))