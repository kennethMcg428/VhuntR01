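; Grabbable item spawner that creates a weapon or object in the grabbing hand, optionally main-hand only or gated by game-mode score.
; Grab spawns the configured class and CastToType forwards the grab to the matching firearm, wand, bow, magazine or projectile Blueprint.
; It then hides its mesh, optionally adds extra magazines and ammo to inventory, and can re-arm on a timer.
; The score gate checks Cost but passes zero to SubractScore.
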(event Custom|ResetTimer
  (bind _skeletalmesh (Variables|Default|GetSkeletalMesh))
  ;[1 1 1] Handle grab and spawning logic
  (Variables|DoNotTouch|SetbCanGrab true)
  (Utilities|Time|ClearandInvalidateTimerbyHandle (stale EventGrab _returnvalue_2))
  (Utilities|IsValid _skeletalmesh
    (:Is%20Valid
      (Rendering|SetVisibility _skeletalmesh true true))))

(event EventBeginPlay
  (bind _skeletalmesh (Variables|Default|GetSkeletalMesh))
  ;[1 1 1] Begin Play
  (if (Variables|SpawnerSetup|GetbStartSpawned)
    (Variables|DoNotTouch|SetbCanGrab true)
    (else
      (Utilities|IsValid _skeletalmesh
        (:Is%20Valid
          (Rendering|SetVisibility _skeletalmesh false true)
          (Variables|DoNotTouch|SetbCanGrab false))))))

(event EventGrab
  (params (Parent :type BP%20VR%20Character%20Object%20Reference) (Hand :type BP%20VR%20Character%20Hand%20Object%20Reference) (AttachPoint :type Scene%20Component%20Object%20Reference))
  (bind _skeletalmesh (Variables|Default|GetSkeletalMesh))
  ;[1 1 1] Handle grab and spawning logic
  (if (Variables|SpawnerSetup|GetbIsMainHandWeapon)
    (if (Variables|/Game/WeaponMaster/Blueprints/Basic/BP_VRCharacterHand.BP_VRCharacterHand_C|GetbIsMainHand Hand)
      (if (Variables|DoNotTouch|GetbCanGrab) :!label _label
        (if (Variables|SurvivalModeSetup|GetbUseGameModeScoreAsCost)
          (bind _asbp_wmgame_mode (Utilities|Casting|CastToBP_WMGameMode (Game|GetGameMode))
            (:then
              (if (>= (Variables|/Game/WeaponMaster/Blueprints/Basic/BP_WMGameMode.BP_WMGameMode_C|GetScore _asbp_wmgame_mode) (Variables|SurvivalModeSetup|GetCost))
                (Default|SubractScore _asbp_wmgame_mode)
                (Variables|DoNotTouch|SetbCanGrab false :!label _label_2)
                (bind _returnvalue (Game|SpawnActorfromClass (Variables|SpawnerSetup|GetSpawnClass) (Transformation|GetWorldTransform AttachPoint) "AlwaysSpawn" 0 true 0))
                (CallFunction|CasttoType _returnvalue Parent Hand AttachPoint)
                (Utilities|IsValid _skeletalmesh
                  (:Is%20Valid
                    (Rendering|SetVisibility _skeletalmesh false true))
                  (:Is%20Not%20Valid
                    _))
                (CallFunction|AddExtratoInventory Parent)
                (if (Variables|SpawnerSetup|GetbAllowRespawn)
                  (bind _returnvalue_2 (Utilities|Time|SetTimerbyEvent (delegate Custom|ResetTimer) (Variables|SpawnerSetup|GetRespawnTime))))))
            (:CastFailed
              (Development|PrintString "NotSurvivalGameMode" false)))
          (else
            (goto _label_2)))))
    (else
      (goto _label))))

(fn ConstructionScript
  (|CallParentFunction))

(fn AddExtratoInventory
  (params (Parent :type BP%20VR%20Character%20Object%20Reference))
  (bind _inventorytriggerfront (Variables|/Game/WeaponMaster/Blueprints/Basic/BP_VRCharacter.BP_VRCharacter_C|GetInventoryTriggerFront Parent))
  (bind _returnvalue (Transformation|GetWorldTransform _inventorytriggerfront))
  (bind (_location _rotation) (Math|Transform|BreakTransform _returnvalue))
  ;[1 1 1] Add extra ammo to inventory
  (Utilities|FlowControl|Sequence
    (:then_0
      (if (Math|Boolean|ANDBoolean (Variables|SurvivalModeSetup|GetbAddExtraMagsToInventory) (Utilities|IsValidClass (Variables|SurvivalModeSetup|GetExtraMagClass)) (> (Variables|SurvivalModeSetup|GetMagsToAddToAddToInventory) 0))
        (for _index (range 1 (Variables|SurvivalModeSetup|GetMagsToAddToAddToInventory))
          (bind _returnvalue_2 (Game|SpawnActorfromClass (Variables|SurvivalModeSetup|GetExtraMagClass) (Math|Transform|MakeTransform _location _rotation) "AlwaysSpawn" 0 0 false 0))
          (Default|InitializeinInventory _returnvalue_2 _inventorytriggerfront Parent))))
    (:then_1
      (if (Variables|SurvivalModeSetup|GetbAddExtraBulletsToInventory)
        (Default|AddAmmo Parent (Variables|SurvivalModeSetup|GetBulletsToAddToInventory) (Variables|SurvivalModeSetup|GetExtraAmmoType))))))

(fn CasttoType
  (params (InteractionObject :type BP%20Interaction%20Object%20Object%20Reference) (Parent :type BP%20VR%20Character%20Object%20Reference) (Hand :type BP%20VR%20Character%20Hand%20Object%20Reference) (AttachPoint :type Scene%20Component%20Object%20Reference))
  ;[1 1 1] Get the appropriate type and call grab function
  (LocalVariables|SetLocalHand Hand)
  (LocalVariables|SetLocalParent Parent)
  (LocalVariables|SetLocalAttachPoint AttachPoint)
  (switch Utilities|FlowControl|Switch|SwitchonEnum_ObjectTypes (Variables|/Game/WeaponMaster/Blueprints/Basic/BP_InteractionObject.BP_InteractionObject_C|GetObjectType InteractionObject)
    (:NewEnumerator0
      (bind _asbp_advanced_firearm (Utilities|Casting|CastToBP_AdvancedFirearm InteractionObject)
        (:then
          (Default|Grab _asbp_advanced_firearm (LocalVariables|GetLocalParent) (LocalVariables|GetLocalHand) (LocalVariables|GetLocalAttachPoint)))
        (:CastFailed
          (Development|PrintString "Not PhysMagWeap" false))))
    (:NewEnumerator1
      (bind _asbp_simple_firearm (Utilities|Casting|CastToBP_SimpleFirearm InteractionObject)
        (:then
          (Default|Grab _asbp_simple_firearm (LocalVariables|GetLocalParent) (LocalVariables|GetLocalHand) (LocalVariables|GetLocalAttachPoint)))
        (:CastFailed
          (Development|PrintString "Not SimpleFirearm" false))))
    (:NewEnumerator6
      (bind _asbp_wand (Utilities|Casting|CastToBP_Wand InteractionObject)
        (:then
          (Default|Grab _asbp_wand (LocalVariables|GetLocalParent) (LocalVariables|GetLocalHand) (LocalVariables|GetLocalAttachPoint)))
        (:CastFailed
          (Development|PrintString "Not Wand" false))))
    (:NewEnumerator8
      (bind _asbp_bow_weapon (Utilities|Casting|CastToBP_BowWeapon InteractionObject)
        (:then
          (Default|Grab _asbp_bow_weapon (LocalVariables|GetLocalParent) (LocalVariables|GetLocalHand) (LocalVariables|GetLocalAttachPoint)))
        (:CastFailed
          (Development|PrintString "Not Bow Weapon" false))))
    (:NewEnumerator7
      (bind _asbp_magazine (Utilities|Casting|CastToBP_Magazine InteractionObject)
        (:then
          (Default|Grab _asbp_magazine (LocalVariables|GetLocalParent) (LocalVariables|GetLocalHand) (LocalVariables|GetLocalAttachPoint)))
        (:CastFailed
          (bind _asbp_held_projectile (Utilities|Casting|CastToBP_HeldProjectile InteractionObject)
            (:then
              (Default|Grab _asbp_held_projectile (LocalVariables|GetLocalParent) (LocalVariables|GetLocalHand) (LocalVariables|GetLocalAttachPoint)))
            (:CastFailed
              (Development|PrintString "Not Held Projectile" false))))))))