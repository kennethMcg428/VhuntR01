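; Base static mesh pickup that VR hands can grab and release, part of a weapon system.
; Grab snaps the root to the hand's attach point, stops physics, reattaches the mesh and applies held offsets, optionally hiding the hand mesh.
; It also registers itself as the hand's attached actor, clears that side's temporary unholster reference and refreshes the magazine counter.
; Release clears these links, shows the hand, detaches and restores collision and physics.
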(event EventGrab
  (params (Parent :type BP%20VR%20Character%20Object%20Reference) (Hand :type BP%20VR%20Character%20Hand%20Object%20Reference) (AttachPoint :type Scene%20Component%20Object%20Reference))
  ;[1 1 1] Hand Grab Logic
  (CallFunction|AttachtoHand Parent Hand AttachPoint))

(event EventReleaseObject
  ;[1 1 1] Hand Release Logic
  (CallFunction|DetachfromHand))

(fn ConstructionScript
  (|CallParentFunction))

(fn AttachtoHand
  (params (Parent :type BP%20VR%20Character%20Object%20Reference) (HandMesh :type BP%20VR%20Character%20Hand%20Object%20Reference) (AttachPoint :type Scene%20Component%20Object%20Reference))
  (bind _staticmesh (Variables|Default|GetStaticMesh))
  ;[1 1 1] Attach To Hand
  (Utilities|IsValid Parent
    (:Is%20Valid
      ;;[0 0 0] SetParentandHandParent
      (Variables|Default|SetParent Parent)
      (Variables|Default|SetParentHand HandMesh)
      (bind _output_get (Variables|Default|SetAttachPoint AttachPoint))
      ;;[0 0 0] Attach and Turn off Physics
      (Transformation|AttachComponentToComponent (Variables|Default|GetRoot) _output_get "None" "SnapToTarget" "SnapToTarget" "KeepWorld" false)
      (Physics|SetSimulatePhysics _staticmesh false)
      (Transformation|AttachComponentToComponent _staticmesh (Variables|Default|GetRoot) "None" "KeepWorld" "KeepWorld" "KeepWorld" false)
      ;;[0 0 0] Set hand attached actor
      (Variables|/Game/WeaponMaster/VirtualRealityBP/Blueprints/BP_MotionController.BP_MotionController_C|SetAttachedActor (Variables|Default|GetParentHand) self)
      ;;[0 0 0] Clear unholster variables
      (switch Utilities|FlowControl|Switch|SwitchonEControllerHand (Variables|/Game/WeaponMaster/VirtualRealityBP/Blueprints/BP_MotionController.BP_MotionController_C|GetHand (Variables|Default|GetParentHand))
        (:Left
          (Variables|/Game/WeaponMaster/Blueprints/Basic/BP_VRCharacter.BP_VRCharacter_C|SetTempLeftUnholsterObject (Variables|Default|GetParent) 0))
        (:Right
          (Variables|/Game/WeaponMaster/Blueprints/Basic/BP_VRCharacter.BP_VRCharacter_C|SetTempRightUnholsterObject (Variables|Default|GetParent) 0)))
      ;;[0 0 0] Do location and rotation adjustments
      (Transformation|SetRelativeLocationAndRotation (Variables|Default|GetStaticMesh) (Variables|Default|GetHeldLocationAdjustment) (Variables|Default|GetHeldRotationAdjustment) false false)
      ;;[0 0 0] Update UI, clear HeldinOffHand, and hide Hand Parent Mesh if desired.
      (Default|UpdateMagCounter (Variables|Default|GetParent))
      (if (Variables|Default|GetbHideInGameHand)
        (Rendering|SetVisibility (Variables|/Game/WeaponMaster/VirtualRealityBP/Blueprints/BP_MotionController.BP_MotionController_C|GetHandMesh (Variables|Default|GetParentHand)) false false)))))

(fn DetachfromHand
  (bind _staticmesh (Variables|Default|GetStaticMesh))
  ;[1 1 1] Detach from hand.
  (Utilities|IsValid (Variables|Default|GetParentHand)
    (:Is%20Valid
      ;;[0 0 0] Clear Attached Actor
      (Variables|/Game/WeaponMaster/VirtualRealityBP/Blueprints/BP_MotionController.BP_MotionController_C|SetAttachedActor (Variables|Default|GetParentHand) 0)
      ;;[0 0 0] Update UI and Show Parent Hand Mesh
      (Default|UpdateMagCounter (Variables|Default|GetParent))
      (Rendering|SetVisibility (Variables|/Game/WeaponMaster/VirtualRealityBP/Blueprints/BP_MotionController.BP_MotionController_C|GetHandMesh (Variables|Default|GetParentHand)) true false)
      ;;[0 0 0] Clear variables
      (Variables|Default|SetParent 0)
      (Variables|Default|SetParentHand 0)
      (Variables|Default|SetAttachPoint 0)
      ;;[0 0 0] Detach from Hand, turn on collision and turn on simulate physics
      (Transformation|DetachFromComponent (Variables|Default|GetRoot) "KeepWorld" "KeepWorld" "KeepWorld" true)
      (Collision|SetCollisionEnabled _staticmesh "QueryAndPhysics")
      (Physics|SetSimulatePhysics _staticmesh true))))