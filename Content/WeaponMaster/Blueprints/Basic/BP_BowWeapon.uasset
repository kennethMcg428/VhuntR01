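; VR bow weapon that can be gripped, holstered, drawn by hand and fired.
; Overlapping a held arrow of the matching class nocks it, going straight into a pull if grip is still held.
; Tick converts motion controller offset into normalized draw, which scales looping rumble and decays after release.
; Releasing past a minimum draw arms the shot; the animation blueprint calls Fire, spawning a projectile with draw-scaled velocity.
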(event OnComponentBeginOverlap(SlideStartVolume)
  (params (OverlappedComponent :type Primitive%20Component%20Object%20Reference) (OtherActor :type Actor%20Object%20Reference) (OtherComp :type Primitive%20Component%20Object%20Reference) (OtherBodyIndex :type Integer) (bFromSweep :type Boolean) (SweepResult :type Hit%20Result%20Structure%20%28by%20ref%29))
  ;[1 1 1] Overlap and allow string pull if grip is still held. (For quick firing)
  ;;[0 0 0] Make sure an arrow isn't nocked
  (if (not (Variables|DoNotTouch|GetbArrowNocked))
    ;;[0 0 0] If correct held object then nock the arrow
    (bind _asbp_held_projectile (Utilities|Casting|CastToBP_HeldProjectile OtherActor)
      (:then
        (Utilities|IsValid (Variables|/Game/WeaponMaster/Blueprints/Basic/BP_InteractionObject.BP_InteractionObject_C|GetParent _asbp_held_projectile)
          (:Is%20Valid
            (Utilities|IsValid (Variables|/Game/WeaponMaster/Blueprints/Basic/BP_InteractionObject.BP_InteractionObject_C|GetParentHand _asbp_held_projectile)
              (:Is%20Valid
                (if (== (Utilities|GetClass _asbp_held_projectile) (Variables|WeaponSetup|GetArrowClass))
                  (CallFunction|NockArrow)
                  ;;[0 0 0] Is trigger still held?
                  (if (Variables|/Game/WeaponMaster/VirtualRealityBP/Blueprints/BP_MotionController.BP_MotionController_C|GetbWantsToGrip (Variables|/Game/WeaponMaster/Blueprints/Basic/BP_InteractionObject.BP_InteractionObject_C|GetParentHand _asbp_held_projectile))
                    ;;[0 0 0] Set slide difference before destroying the bullet.
                    (CallFunction|SetSlideDifference (Variables|/Game/WeaponMaster/Blueprints/Basic/BP_InteractionObject.BP_InteractionObject_C|GetParentHand _asbp_held_projectile))
                    (Default|DestroyBullet _asbp_held_projectile true))))))))
      (:CastFailed
        (Development|PrintString "Not held Projectile" false)))))

(event Custom|Fire
  ;[1 1 1] Fire arrow, called by animation blueprint
  (if (and (Variables|DoNotTouch|GetbCanFire) (Variables|DoNotTouch|GetbArrowNocked))
    (Variables|DoNotTouch|SetbCanFire false)
    (Variables|DoNotTouch|SetbReleased false)
    (Variables|DoNotTouch|SetbArrowNocked false)
    (Default|ControllerRumble (Variables|Default|GetParentHand) (Variables|WeaponRumbleSetup|GetFireIntensity) (Variables|WeaponRumbleSetup|GetFireDuration))
    (Rendering|SetVisibility (Variables|Default|GetArrow) false false)
    (CallFunction|SpawnArrow)))

(event Custom|StartRumbleTimer
  ;[1 1 1] Rumble TImer
  (bind _returnvalue (Utilities|Time|SetTimerbyEvent (delegate Custom|RumbleTimer) 0.05 true)))

(event Custom|RumbleTimer
  (bind _slidepositiondifference (Variables|DoNotTouch|GetSlidePositionDifference))
  (bind _interactioncomponent (Variables|DoNotTouch|GetInteractionComponent))
  ;[1 1 1] Rumble TImer
  (Utilities|IsValid _interactioncomponent
    (:Is%20Valid
      (Default|LoopRumbleController _interactioncomponent (* (Variables|WeaponRumbleSetup|GetMaxPullIntensity) _slidepositiondifference) (* (Variables|WeaponRumbleSetup|GetMaxPullDuration) _slidepositiondifference)))))

(event Custom|StopRumbleTimer
  ;[1 1 1] Rumble TImer
  (Utilities|Time|ClearandInvalidateTimerbyHandle (stale Custom|StartRumbleTimer _returnvalue)))

(event EventBeginPlay
  ;[1 1 1] Begin Play
  (Rendering|SetVisibility (Variables|Default|GetArrow) false false)
  (Utilities|IsValid (Variables|Default|GetParent)
    (:Is%20Valid
      (Physics|SetSimulatePhysics (Variables|Default|GetSkeletalMesh) false)
      (Actor|Tick|SetActorTickEnabled true))
    (:Is%20Not%20Valid
      (Physics|SetSimulatePhysics (Variables|Default|GetSkeletalMesh) true)
      (Actor|Tick|SetActorTickEnabled false))))

(event EventReleaseObject
  ;[1 1 1] Grip Events
  (|CallParentFunction)
  (Variables|DoNotTouch|SetbAttachedToHand false)
  (Actor|Tick|SetActorTickEnabled false))

(event EventTick
  (params (DeltaSeconds :type Float%20%28single-precision%29))
  (bind _pulladjust (Variables|WeaponAdjustments|GetPullAdjust))
  (bind _slidegrabvolume (Variables|Default|GetSlideGrabVolume))
  (bind _slidestartvolume (Variables|Default|GetSlideStartVolume))
  (bind _interactioncomponent (Variables|DoNotTouch|GetInteractionComponent))
  (bind _maxslidedistance (Variables|WeaponSetup|GetMaxSlideDistance))
  (bind _returnvalue (Transformation|GetRelativeTransform _slidestartvolume))
  (bind _returnvalue_2 (Transformation|GetRelativeTransform _slidegrabvolume))
  (bind _location (Math|Transform|BreakTransform _returnvalue))
  (bind _location_2 (Math|Transform|BreakTransform _returnvalue_2))
  (bind _returnvalue_3 (- _location_2 _location))
  (bind _x (Math|Vector|BreakVector _returnvalue_3))
  (bind _returnvalue_4 (- _x _pulladjust))
  ;[1 1 1] Handle Manual manipulation of the bow string
  (if (not (Variables|DoNotTouch|GetbGrabbed))
    (if (> (Variables|DoNotTouch|GetSlidePositionDifference) 0.0001)
      (Variables|DoNotTouch|SetSlidePositionDifference (- (Variables|DoNotTouch|GetSlidePositionDifference) (* DeltaSeconds 25.0)))
      (else
        (Variables|DoNotTouch|SetSlidePositionDifference 0.0)))
    (else
      (Utilities|IsValid _interactioncomponent
        (:Is%20Valid
          (Transformation|SetWorldLocation (Variables|Default|GetSlideGrabVolume) (- (Transformation|GetWorldLocation (Variables|/Game/WeaponMaster/VirtualRealityBP/Blueprints/BP_MotionController.BP_MotionController_C|GetMotionController _interactioncomponent)) (Variables|DoNotTouch|GetSlideStartDifference)) false false)
          (if (>= _returnvalue_4 0.0)
            (Variables|DoNotTouch|SetSlidePositionDifference 0.0)
            (else
              (Variables|DoNotTouch|SetSlidePositionDifference (/ (Math|Float|Min(Float) (Math|Float|Absolute(Float) _returnvalue_4) _maxslidedistance) _maxslidedistance)))))))))

(event EventInteract
  (params (Hand :type BP%20VR%20Character%20Hand%20Object%20Reference))
  ;[1 1 1] Trigger Interactions
  (Utilities|IsValid (Variables|Default|GetParent)
    (:Is%20Valid
      (CallFunction|SetSlideDifference Hand))))

(event EventStopInteraction
  ;[1 1 1] Trigger Interactions
  (CallFunction|EndInteraction))

(event EventGrab
  (params (Parent :type BP%20VR%20Character%20Object%20Reference) (Hand :type BP%20VR%20Character%20Hand%20Object%20Reference) (AttachPoint :type Scene%20Component%20Object%20Reference))
  ;[1 1 1] Grip Events
  (Utilities|IsValid (Variables|Default|GetParent)
    (:Is%20Not%20Valid
      (|CallParentFunction Parent Hand AttachPoint)
      (Variables|DoNotTouch|SetbAttachedToHand true)
      (Actor|Tick|SetActorTickEnabled true))))

(event EventHolster
  (params (HolsterComponent :type Skeletal%20Mesh%20Component%20Object%20Reference) (AttachPoint :type Scene%20Component%20Object%20Reference))
  ;[1 1 1] Grip Events
  (CallFunction|ReleaseObject)
  (CallFunction|AttachtoHolster HolsterComponent AttachPoint)
  (Actor|Tick|SetActorTickEnabled false))

(event EventUnHolster
  (params (Parent :type BP%20VR%20Character%20Object%20Reference) (Hand :type BP%20VR%20Character%20Hand%20Object%20Reference) (AttachPoint :type Scene%20Component%20Object%20Reference))
  ;[1 1 1] Grip Events
  (CallFunction|DetachfromHolster)
  (CallFunction|Grab Parent Hand AttachPoint)
  (Actor|Tick|SetActorTickEnabled true))

(fn ConstructionScript
  ;[1 1 1] Call to parent Contstruction
  (|CallParentFunction)
  ;[1 1 1] Attach Components to correct sockets
  (Utilities|FlowControl|Sequence
    (:then_0
      (Transformation|AttachComponentToComponent (Variables|Default|GetSlideGrabVolume) (Variables|Default|GetSkeletalMesh) (Variables|WeaponSetup|GetInteractionSocket) "SnapToTarget" "SnapToTarget" "KeepWorld" true))
    (:then_1
      (Transformation|AttachComponentToComponent (Variables|Default|GetSlideStartVolume) (Variables|Default|GetSkeletalMesh) (Variables|WeaponSetup|GetInteractionSocket) "SnapToTarget" "SnapToTarget" "KeepWorld" true))
    (:then_2
      (Transformation|AttachComponentToComponent (Variables|Default|GetArrow) (Variables|Default|GetSkeletalMesh) (Variables|WeaponSetup|GetNockSocket) "SnapToTarget" "SnapToTarget" "KeepWorld" true))
    (:then_3
      (Transformation|AttachComponentToComponent (Variables|Default|GetFireVolume) (Variables|Default|GetSkeletalMesh) (Variables|WeaponSetup|GetFireSocket) "SnapToTarget" "SnapToTarget" "KeepWorld" true))))

(fn SetSlideDifference
  (params (Hand :type BP%20VR%20Character%20Hand%20Object%20Reference))
  ;[1 1 1] Set the difference between the hand position and the slide start position
  (Variables|DoNotTouch|SetInteractionComponent Hand)
  (Rendering|SetVisibility (Variables|/Game/WeaponMaster/VirtualRealityBP/Blueprints/BP_MotionController.BP_MotionController_C|GetHandMesh Hand) false false)
  (Variables|DoNotTouch|SetSlideStartDifference (- (Transformation|GetWorldLocation (Variables|/Game/WeaponMaster/VirtualRealityBP/Blueprints/BP_MotionController.BP_MotionController_C|GetMotionController Hand)) (Transformation|GetWorldLocation (Variables|Default|GetSlideGrabVolume))))
  (Variables|DoNotTouch|SetbGrabbed true)
  (CallFunction|StartRumbleTimer))

(fn EndInteraction
  ;[1 1 1] Fire Arrow
  ;;[1 1 1] If we have pulled back far enough (.2) then set canfire to true
  (bind _output_get (Variables|DoNotTouch|SetProjectileModifier (Variables|DoNotTouch|GetSlidePositionDifference)))
  (if (and (>= _output_get 0.2) (Variables|DoNotTouch|GetbArrowNocked))
    (Variables|DoNotTouch|SetbCanFire true))
  ;;[1 1 1] Set the interaction Socket location to the slide grab volume
  (Transformation|SetWorldLocation (Variables|Default|GetSlideGrabVolume) (Transformation|GetSocketLocation (Variables|Default|GetSkeletalMesh) (Variables|WeaponSetup|GetInteractionSocket)) false false)
  ;;[1 1 1] Show hand if there is an interaction component
  (Utilities|IsValid (Variables|DoNotTouch|GetInteractionComponent)
    (:Is%20Valid
      (Rendering|SetVisibility (Variables|/Game/WeaponMaster/VirtualRealityBP/Blueprints/BP_MotionController.BP_MotionController_C|GetHandMesh (Variables|DoNotTouch|GetInteractionComponent)) true false))
    (:Is%20Not%20Valid
      _))
  ;;[1 1 1] Clear Variables
  (Variables|DoNotTouch|SetbGrabbed false)
  (Variables|DoNotTouch|SetSlideStartDifference "0, 0, 0")
  ;;[1 1 1] If ther is an interaction component stop rumble timer and clear it
  (Utilities|IsValid (Variables|DoNotTouch|GetInteractionComponent)
    (:Is%20Valid
      (CallFunction|StopRumbleTimer)
      (Variables|DoNotTouch|SetInteractionComponent 0))))

(fn SpawnArrow
  (bind _muzzlesocket (Variables|WeaponSetup|GetMuzzleSocket))
  (bind _skeletalmesh (Variables|Default|GetSkeletalMesh))
  (bind _returnvalue (Transformation|GetSocketTransform _skeletalmesh _muzzlesocket "RTS_World"))
  ;[1 1 1] Spawn Arrow and pass in variables
  (Game|SpawnActorfromClass (Variables|WeaponSetup|GetProjectileType) _returnvalue "AlwaysSpawn" self "0.000000,0.000000,0.000000" "0.000000,0.000000,0.000000" (.Rotation (Math|Transform|BreakTransform _returnvalue)) 0.0 true false (Variables|DoNotTouch|GetProjectileModifier) (Variables|Default|GetParent))
  (return))

(fn NockArrow
  ;[1 1 1] Nock the arrow by showing the Arrow component and playing a sound.
  (Rendering|SetVisibility (Variables|Default|GetArrow) true false)
  (Variables|DoNotTouch|SetbArrowNocked true)
  (Audio|PlaySoundatLocation (Variables|WeaponSounds|GetNockArrowSound) (Transformation|GetWorldLocation (Variables|Default|GetSkeletalMesh)))
  (return))

(fn AttachtoHolster
  (params (HolsterComponent :type Skeletal%20Mesh%20Component%20Object%20Reference) (AttachPoint :type Scene%20Component%20Object%20Reference))
  ;[1 1 1] Attach to Holster
  (Utilities|IsValid HolsterComponent
    (:Is%20Valid
      (Utilities|IsValid AttachPoint
        (:Is%20Valid
          ;;[0 0 0] SetHolsterParent
          (Variables|Default|SetHolsterParent HolsterComponent)
          (bind _output_get (Variables|Default|SetAttachPoint AttachPoint))
          ;;[0 0 0] Turn off Physics
          (Physics|SetSimulatePhysics (Variables|Default|GetSkeletalMesh) false)
          ;;[0 0 0] Turn  off overlap events so we cannot grab.
          (Variables|/Script/Engine.PrimitiveComponent|SetbGenerateOverlapEvents (Variables|Default|GetSkeletalMesh) false)
          ;;[0 0 0] Attach to Holster and set location and rotation adjustments
          (Transformation|AttachComponentToComponent (Variables|Default|GetRoot) _output_get "None" "SnapToTarget" "SnapToTarget" "KeepWorld" false)
          (Transformation|AttachComponentToComponent (Variables|Default|GetSkeletalMesh) (Variables|Default|GetRoot) "None" "SnapToTarget" "SnapToTarget" "KeepWorld" false)
          (Transformation|SetRelativeLocationAndRotation (Variables|Default|GetSkeletalMesh) (Variables|Default|GetHolsterLocationAdjustment) (Variables|Default|GetHolsterRotationAdjustment) false false)
          ;;[0 0 0] Play Sound
          (Audio|PlaySoundatLocation (Variables|WeaponSounds|GetHolsterSound) (Transformation|GetWorldLocation (Variables|Default|GetSkeletalMesh)))
          ;;[0 0 0] Clear Varaible
          (Variables|Default|SetParentHand 0))))))

(fn DetachfromHolster
  ;[1 1 1] Detach from holster and clear variables
  (Transformation|DetachFromComponent (Variables|Default|GetRoot) "KeepWorld" "KeepWorld" "KeepWorld" false)
  ;;[0 0 0] Turn on overlap events so we can grab again
  (Variables|/Script/Engine.PrimitiveComponent|SetbGenerateOverlapEvents (Variables|Default|GetSkeletalMesh) true)
  (Variables|Default|SetHolsterParent 0)
  (Variables|Default|SetAttachPoint 0))