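; BP_Wand is a grabbable wand weapon that charges a spell projectile while the trigger is held and fires it on release.
; Trigger press spawns a small projectile attached to the muzzle socket, and a looping timer grows its scale and PowerModifier while held in hand, up to a cap.
; Release stops the timer, passes the power as damage modifier, detaches the projectile, activates its movement and resets the charge.
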(event Custom|GrowTimerStart
  ;[1 1 1] Grow Timer (interval at which the spell grows again)
  (bind _returnvalue (Utilities|Time|SetTimerbyEvent (delegate Custom|GrowSpell) 0.02 true)))

(event Custom|GrowSpell
  (bind _incrementvalue (Variables|WandSetup|GetIncrementValue))
  (bind _currentprojectile (Variables|DoNotTouch|GetCurrentProjectile))
  ;[1 1 1] Grow the spells size and power over time while the trigger is held down.
  (if (and (Variables|DoNotTouch|GetbAttachedToHand) (<= (Variables|DoNotTouch|GetPowerModifier) 1.0))
    (Variables|DoNotTouch|SetPowerModifier (+ (Variables|DoNotTouch|GetPowerModifier) (Variables|WandSetup|GetIncrementValue)))
    (Variables|DoNotTouch|SetScale (Math|Vector|MakeVector (+ (.X (Math|Vector|BreakVector (Variables|DoNotTouch|GetScale))) _incrementvalue) (+ (.Y (Math|Vector|BreakVector (Variables|DoNotTouch|GetScale))) _incrementvalue) (+ (.Z (Math|Vector|BreakVector (Variables|DoNotTouch|GetScale))) _incrementvalue)))
    (Utilities|IsValid _currentprojectile
      (:Is%20Valid
        (Transformation|SetWorldScale3D (Variables|/Game/WeaponMaster/Blueprints/Basic/BP_ChamberedBulletBase.BP_ChamberedBulletBase_C|GetSphere _currentprojectile) (Variables|DoNotTouch|GetScale))))
    (else
      (CallFunction|GrowTimerStop))))

(event Custom|GrowTimerStop
  ;[1 1 1] Grow Timer (interval at which the spell grows again)
  (Utilities|Time|ClearandInvalidateTimerbyHandle (stale Custom|GrowTimerStart _returnvalue)))

(event EventBeginPlay
  (bind _skeletalmesh (Variables|Default|GetSkeletalMesh))
  ;[1 1 1] Begin Play
  (Utilities|IsValid (Variables|Default|GetParent)
    (:Is%20Valid
      (Physics|SetSimulatePhysics _skeletalmesh false))
    (:Is%20Not%20Valid
      (Physics|SetSimulatePhysics _skeletalmesh true))))

(event EventReleaseObject
  ;[1 1 1] Hand Release Loggic
  (|CallParentFunction)
  (Variables|DoNotTouch|SetbAttachedToHand false))

(event EventTriggeron
  ;[1 1 1] Start Spell
  (CallFunction|StartSpell))

(event EventTriggerOff
  ;[1 1 1] Stop and fire spell
  (CallFunction|GrowTimerStop)
  (CallFunction|FireSpell))

(event EventGrab
  (params (Parent :type BP%20VR%20Character%20Object%20Reference) (Hand :type BP%20VR%20Character%20Hand%20Object%20Reference) (AttachPoint :type Scene%20Component%20Object%20Reference))
  ;[1 1 1] Hand Grab Logic
  (Utilities|IsValid (Variables|Default|GetParent)
    (:Is%20Not%20Valid
      (|CallParentFunction Parent Hand AttachPoint)
      (Variables|DoNotTouch|SetbAttachedToHand true))))

(fn ConstructionScript
  (|CallParentFunction))

(fn StartSpell
  (bind _muzzlesocket (Variables|WandSetup|GetMuzzleSocket))
  (bind _skeletalmesh (Variables|Default|GetSkeletalMesh))
  (bind _returnvalue (Transformation|GetSocketTransform _skeletalmesh _muzzlesocket "RTS_World"))
  (bind (_location _rotation) (Math|Transform|BreakTransform _returnvalue))
  ;[1 1 1] Spawn projectile at .1 of its size and attach it to the wand before starting the grow timer.
  (bind _returnvalue_2 (Game|SpawnActorfromClass (Variables|WandSetup|GetProjectileClass) (Math|Transform|MakeTransform _location _rotation "0.100000,0.100000,0.100000") "AlwaysSpawn" self "0.000000,0.000000,0.000000" "0.000000,0.000000,0.000000" "0.000000,0.000000,0.000000" 0.0 false false (Variables|Default|GetParent)))
  (bind _output_get (Variables|DoNotTouch|SetCurrentProjectile _returnvalue_2))
  (Variables|DoNotTouch|SetbSpellAttached true)
  (Transformation|AttachComponentToComponent (Variables|/Game/WeaponMaster/Blueprints/Basic/BP_ChamberedBulletBase.BP_ChamberedBulletBase_C|GetSphere _output_get) (Variables|Default|GetSkeletalMesh) (Variables|WandSetup|GetMuzzleSocket) "SnapToTarget" "SnapToTarget" "KeepRelative" true)
  (CallFunction|GrowTimerStart))

(fn FireSpell
  ;[1 1 1] Detach, and activate projectile
  (Utilities|IsValid (Variables|DoNotTouch|GetCurrentProjectile)
    (:Is%20Valid
      (Variables|/Game/WeaponMaster/Blueprints/Basic/BP_ChamberedBulletBase.BP_ChamberedBulletBase_C|SetWeaponDamageModifier (Variables|DoNotTouch|GetCurrentProjectile) (Variables|DoNotTouch|GetPowerModifier))
      (Transformation|DetachFromComponent (Variables|/Game/WeaponMaster/Blueprints/Basic/BP_ChamberedBulletBase.BP_ChamberedBulletBase_C|GetSphere (Variables|DoNotTouch|GetCurrentProjectile)) "KeepRelative" "KeepRelative" "KeepRelative" true)
      (bind _asbp_projectile (Utilities|Casting|CastToBP_Projectile (Variables|DoNotTouch|GetCurrentProjectile))
        (:then
          (bind _returnvalue (Physics|GetPhysicsLinearVelocity (Variables|/Game/WeaponMaster/Blueprints/Basic/BP_ChamberedBulletBase.BP_ChamberedBulletBase_C|GetSphere _asbp_projectile) "None"))
          (bind _returnvalue_2 (Class|PrimitiveComponent|GetPhysicsAngularVelocity (Variables|/Game/WeaponMaster/Blueprints/Basic/BP_ChamberedBulletBase.BP_ChamberedBulletBase_C|GetSphere _asbp_projectile) "None"))
          (Default|ActivateMovement _asbp_projectile _returnvalue _returnvalue_2)
          (Variables|DoNotTouch|SetCurrentProjectile 0)
          (Variables|DoNotTouch|SetPowerModifier 0.1)
          (Variables|DoNotTouch|SetScale "0.100000,0.100000,0.100000")
          (return))
        (:CastFailed
          (return))))
    (:Is%20Not%20Valid
      (return))))