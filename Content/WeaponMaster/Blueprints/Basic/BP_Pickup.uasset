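; BP_Pickup is an ammo pickup that grants a set amount of a given ammo type to whoever grabs it.
; Grab passes the ammo to the grabbing parent and refreshes its weapon widget, with a CanGrab flag blocking repeat grabs.
; Respawnable pickups hide their mesh and text, then a one-shot timer calls Activate to restore them.
; Non-respawnable pickups destroy themselves.
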(event Custom|Activate
  (bind _staticmesh (Variables|Default|GetStaticMesh))
  ;[1 1 1] Reactivate ammo pickup
  (Utilities|Time|ClearandInvalidateTimerbyHandle (stale EventGrab _returnvalue))
  (Utilities|IsValid _staticmesh
    (:Is%20Valid
      (Rendering|SetVisibility _staticmesh true true)
      (Rendering|SetVisibility (Variables|Default|GetTextRender) true false)
      (Variables|Default|SetParent 0)
      (Variables|Default|SetbCanGrab true))))

(event EventBeginPlay
  ;[1 1 1] begin play
  (Variables|Default|SetbCanGrab true))

(event EventGrab
  (params (Parent :type BP%20VR%20Character%20Object%20Reference) (Hand :type BP%20VR%20Character%20Hand%20Object%20Reference) (AttachPoint :type Scene%20Component%20Object%20Reference))
  (bind _staticmesh (Variables|Default|GetStaticMesh))
  ;[1 1 1] Get player parent and then add the ammo amount
  (if (Variables|Default|GetbCanGrab)
    (Variables|Default|SetbCanGrab false)
    (Variables|Default|SetParent Parent)
    (Default|AddAmmo (Variables|Default|GetParent) (Variables|Default|GetAddAmmoAmount) (Variables|Default|GetAmmoType))
    (Default|UpdateWeaponWidget (Variables|Default|GetParent))
    (if (Variables|Default|GetbCan%20Respawn)
      (Utilities|IsValid _staticmesh
        (:Is%20Valid
          (Rendering|SetVisibility _staticmesh false true)
          (Rendering|SetVisibility (Variables|Default|GetTextRender) false false)
          ;[1 1 1] set reactivation timer
          (bind _returnvalue (Utilities|Time|SetTimerbyEvent (delegate Custom|Activate) (Variables|Default|GetRespawnTime)))))
      (else
        (Actor|DestroyActor)))))

(fn ConstructionScript
  (|CallParentFunction))