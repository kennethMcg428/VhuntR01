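; BP_HeldProjectile is a hand-held ammo round that plays pickup and holster sounds and can be stowed as ammo.
; Grab and release update attachment state, and a drop can start a timed destroy that is cancelled if the round is held or in a magazine when it fires.
; Stowing adds ammo to the parent, restores the hand mesh and destroys the actor.
; DestroyBullet removes it with optional hand unhiding, and a timer clears the ejecting flag.
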(event Custom|StartDestroy
  ;[1 1 1] Destroy Timer
  (bind _returnvalue (Utilities|Time|SetTimerbyEvent (delegate Custom|Destroy) (Variables|HeldProjectileSetup|GetDestroyTimer))))

(event Custom|EjectTimer
  ;[1 1 1] Destroy Timer
  (bind _returnvalue (Utilities|Time|SetTimerbyEvent (delegate Custom|Eject) 1.0)))

(event Custom|Eject
  ;[1 1 1] Destroy Timer
  (Variables|DoNotTouch|SetbEjecting false)
  (Utilities|Time|ClearandInvalidateTimerbyHandle (stale Custom|EjectTimer _returnvalue)))

(event Custom|Destroy
  ;[1 1 1] Destroy Timer
  (if (or (Variables|DoNotTouch|GetbAttachedToHand) (Variables|DoNotTouch|GetbInMagazine))
    (Utilities|Time|ClearandInvalidateTimerbyHandle (stale Custom|StartDestroy _returnvalue))
    (Variables|DoNotTouch|SetbQueuedToDrop false)
    (else
      (Utilities|Time|ClearandInvalidateTimerbyHandle (stale Custom|StartDestroy _returnvalue))
      (Actor|DestroyActor))))

(event EventAddtoInventory
  (params (InventoryObj :type Static%20Mesh%20Component%20Object%20Reference) (Hand :type BP%20VR%20Character%20Hand%20Object%20Reference))
  (bind _parenthand (Variables|Default|GetParentHand))
  ;[1 1 1] Add to inventory
  (Variables|DoNotTouch|SetbAttachedToHand false)
  (Utilities|IsValid (Variables|Default|GetParent)
    (:Is%20Valid
      (Default|AddAmmo (Variables|Default|GetParent) 1 (Variables|Default|GetAmmoType))
      (Rendering|SetVisibility (Variables|/Game/WeaponMaster/VirtualRealityBP/Blueprints/BP_MotionController.BP_MotionController_C|GetHandMesh _parenthand) true false)
      (Variables|/Game/WeaponMaster/VirtualRealityBP/Blueprints/BP_MotionController.BP_MotionController_C|SetAttachedActor _parenthand 0)
      (Variables|Default|SetAttachPoint 0)
      (Variables|Default|SetParent 0)
      (Audio|PlaySoundatLocation (Variables|Sounds|GetHolsterSound) (Transformation|GetWorldLocation (Variables|Default|GetSkeletalMesh)))
      (Actor|DestroyActor))))

(event EventGrab
  (params (Parent :type BP%20VR%20Character%20Object%20Reference) (Hand :type BP%20VR%20Character%20Hand%20Object%20Reference) (AttachPoint :type Scene%20Component%20Object%20Reference))
  ;[1 1 1] Grab
  (|CallParentFunction Parent Hand AttachPoint)
  (Variables|DoNotTouch|SetbAttachedToHand true)
  (Variables|Default|SetbInInventory false)
  (Variables|DoNotTouch|SetInventoryObj 0)
  (Audio|PlaySoundatLocation (Variables|Sounds|GetPickupSound) (Transformation|GetWorldLocation (Variables|Default|GetSkeletalMesh))))

(event EventReleaseObject
  ;[1 1 1] Release
  (|CallParentFunction)
  (Variables|DoNotTouch|SetbAttachedToHand false)
  (if (Math|Boolean|ANDBoolean (Variables|HeldProjectileSetup|GetbDestroyOnDrop) (not (Variables|DoNotTouch|GetbQueuedToDrop)) (not (Variables|DoNotTouch|GetbInMagazine)))
    (Variables|DoNotTouch|SetbQueuedToDrop true)
    (CallFunction|StartDestroy)))

(fn ConstructionScript
  ;[1 1 1] Call to parent construction
  (|CallParentFunction))

(fn DestroyBullet
  (params (KeepHandHidden :type Boolean))
  (bind _parenthand (Variables|Default|GetParentHand))
  ;[1 1 1] Show hand if desired, reset parent hand attached actor, and then destroy the bullet
  (Utilities|IsValid _parenthand
    (:Is%20Valid
      (if (not KeepHandHidden)
        (Rendering|SetVisibility (Variables|/Game/WeaponMaster/VirtualRealityBP/Blueprints/BP_MotionController.BP_MotionController_C|GetHandMesh _parenthand) true false)))
    (:Is%20Not%20Valid
      _))
  (Utilities|IsValid (Variables|Default|GetParent)
    (:Is%20Valid
      (Variables|/Game/WeaponMaster/VirtualRealityBP/Blueprints/BP_MotionController.BP_MotionController_C|SetAttachedActor _parenthand 0))
    (:Is%20Not%20Valid
      _))
  (Actor|DestroyActor))