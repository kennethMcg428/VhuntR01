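; Shooting target actor that scores point-damage hits by how close they land to its centre.
; On point damage it measures the distance from the hit location to its Scene component and steps through concentric distance bands, giving higher scores nearer the centre and zero outside.
; The result is pushed to its WB_HitScore widget component through UpdateInternal, which also resets to zero on begin play.
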(event EventBeginPlay
  ;[1 1 1] Set to 0 on begin play
  (bind _aswb_hit_score (Utilities|Casting|CastToWB_HitScore (UserInterface|GetUserWidgetObject (Variables|Default|GetWidget))))
  (Default|UpdateInternal _aswb_hit_score))

(event Collision|EventActorBeginOverlap
  (params (OtherActor :type Actor%20Object%20Reference)))

(event EventTick
  (params (DeltaSeconds :type Float%20%28single-precision%29)))

(event Game|Damage|EventPointDamage
  (params (Damage :type Float%20%28single-precision%29) (DamageType :type Damage%20Type%20Object%20Reference) (HitLocation :type Vector) (HitNormal :type Vector :default "0, 0, 0") (HitComponent :type Primitive%20Component%20Object%20Reference) (BoneName :type Name :default "None") (ShotFromDirection :type Vector :default "0, 0, 0") (InstigatedBy :type Controller%20Object%20Reference) (DamageCauser :type Actor%20Object%20Reference) (HitInfo :type Hit%20Result%20Structure%20%28by%20ref%29))
  ;[1 1 1] On point damage use distance between locations to get the hit point and decide the score.
  (if (Math|Float|InRange(Float) (Math|Vector|VectorLength (- HitLocation (Transformation|GetWorldLocation (Variables|Default|GetScene)))) 0.0 1e+01)
    (bind _aswb_hit_score (Utilities|Casting|CastToWB_HitScore (UserInterface|GetUserWidgetObject (Variables|Default|GetWidget))))
    (Default|UpdateInternal _aswb_hit_score 100)
    (elif (Math|Float|InRange(Float) (Math|Vector|VectorLength (- HitLocation (Transformation|GetWorldLocation (Variables|Default|GetScene)))) 1e+01 25.0)
      (bind _aswb_hit_score_2 (Utilities|Casting|CastToWB_HitScore (UserInterface|GetUserWidgetObject (Variables|Default|GetWidget))))
      (Default|UpdateInternal _aswb_hit_score_2 80)
      (elif (Math|Float|InRange(Float) (Math|Vector|VectorLength (- HitLocation (Transformation|GetWorldLocation (Variables|Default|GetScene)))) 25.0 4e+01)
        (bind _aswb_hit_score_3 (Utilities|Casting|CastToWB_HitScore (UserInterface|GetUserWidgetObject (Variables|Default|GetWidget))))
        (Default|UpdateInternal _aswb_hit_score_3 60)
        (elif (Math|Float|InRange(Float) (Math|Vector|VectorLength (- HitLocation (Transformation|GetWorldLocation (Variables|Default|GetScene)))) 4e+01 55.0)
          (bind _aswb_hit_score_4 (Utilities|Casting|CastToWB_HitScore (UserInterface|GetUserWidgetObject (Variables|Default|GetWidget))))
          (Default|UpdateInternal _aswb_hit_score_4 40)
          (elif (Math|Float|InRange(Float) (Math|Vector|VectorLength (- HitLocation (Transformation|GetWorldLocation (Variables|Default|GetScene)))) 55.0 7e+01)
            (bind _aswb_hit_score_5 (Utilities|Casting|CastToWB_HitScore (UserInterface|GetUserWidgetObject (Variables|Default|GetWidget))))
            (Default|UpdateInternal _aswb_hit_score_5 20)
            (else
              (bind _aswb_hit_score_6 (Utilities|Casting|CastToWB_HitScore (UserInterface|GetUserWidgetObject (Variables|Default|GetWidget))))
              (Default|UpdateInternal _aswb_hit_score_6))))))))

(fn ConstructionScript)